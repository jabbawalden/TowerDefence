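; Blueprint function library of shared gameplay helpers for combat damage, enemy status checks and player action sounds.
; DealDamageToActor subtracts typed damage from the target's health component, scaling pierce and blunt by resistances, then calls CheckLife.
; CheckIfAfflicted casts through three enemy classes to report affliction and virus-damage eligibility.
; Play3DSound plays a sound selected from a sound struct at a location; CheckIfSlowedDown is an empty stub.
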(fn `CheckIfAfflicted`
  (params (Actor :type "Actor Object Reference"))
  (returns (IsAfflicted :type Boolean) (CanVirusDamage :type Boolean))
  (locals (Afflicted :type Boolean))
  (bind _afflicted (`local.Afflicted`))
  (`/Engine/EditorBlueprintResources/StandardMacros.IsValid` Actor
    (:`Is Valid`
      (bind _asbp_ai_enemy_one (cast `/Game/Classes/AI/BP_AI_EnemyOne` Actor)
        (:`then`
          (set `local.Afflicted` (> (`/Game/Classes/AI/BP_AI_EnemyOne.AfflictedCounter` _asbp_ai_enemy_one) 0))
          (return _afflicted (`/Game/Classes/AI/BP_AI_EnemyOne.CanVirusDamage` _asbp_ai_enemy_one)))
        (:`CastFailed`
          (bind _asbp_ai_enemy_two (cast `/Game/Classes/AI/BP_AI_EnemyTwo` Actor)
            (:`then`
              (set `local.Afflicted` (> (`/Game/Classes/AI/BP_AI_EnemyTwo.AfflictedCounter` _asbp_ai_enemy_two) 0))
              (return _afflicted (`/Game/Classes/AI/BP_AI_EnemyTwo.Can Virus Damage` _asbp_ai_enemy_two)))
            (:`CastFailed`
              (bind _asbp_ai_enemy_three (cast `/Game/Classes/AI/BP_AI_EnemyThree` Actor))
              (set `local.Afflicted` (> (`/Game/Classes/AI/BP_AI_EnemyThree.AfflictedCounter` _asbp_ai_enemy_three) 0))
              (return _afflicted (`/Game/Classes/AI/BP_AI_EnemyThree.Can Virus Damage` _asbp_ai_enemy_three)))))))))

(fn `CheckIfSlowedDown`)

(fn `Deal Damage To Actor`
  (params (Actor :type "Actor Object Reference") (Damage :type "Float (double-precision)") (`Pierce Damage` :type "Float (double-precision)") (`Blunt Damage` :type "Float (double-precision)") (`Virus Damage` :type "Float (double-precision)"))
  (locals (PercentCheck :type "Float (double-precision)" :default 1.0))
  (bind _returnvalue (`Actor.GetComponentByClass` Actor "/Game/Classes/Components/CBP_HealthComponent.CBP_HealthComponent_C"))
  (`/Engine/EditorBlueprintResources/StandardMacros.IsValid` Actor
    (:`Is Valid`
      (set `/Game/Classes/Components/CBP_HealthComponent.Health` (- (`/Game/Classes/Components/CBP_HealthComponent.Health` _returnvalue) (+ Damage (* `Pierce Damage` (- (`local.PercentCheck`) (`/Game/Classes/Components/CBP_HealthComponent.Pierce Resistance` _returnvalue))) (* `Blunt Damage` (- (`local.PercentCheck`) (`/Game/Classes/Components/CBP_HealthComponent.Blunt Resistance` _returnvalue))) `Virus Damage`)) _returnvalue)
      (`/Game/Classes/Components/CBP_HealthComponent.CheckLife` _returnvalue))))

(fn `Play 3D Sound`
  (params (Location :type "Vector Structure"))
  (locals (SoundStruct :type "/Game/Classes/GameFiles/SBP_PlayerAudio Structure"))
  (bind (_player_lightmeleeattack _player_heavymeleeattack _player_bowattack _player_stealthin _playerstealthout) (break `/Game/Classes/GameFiles/SBP_PlayerAudio` (`local.SoundStruct`)))
  (`GameplayStatics.PlaySoundAtLocation` null (select `/Game/Classes/GameFiles/Enum_PlayerState` "NewEnumerator0" :`NewEnumerator0` _player_lightmeleeattack :`NewEnumerator1` _player_heavymeleeattack :`NewEnumerator2` _player_bowattack :`NewEnumerator3` _player_stealthin :`NewEnumerator4` _playerstealthout) Location (struct) 1.0 1.0 0.0 null null null))