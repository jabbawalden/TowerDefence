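; Main game mode that holds the state for a wave-based enemy spawning game.
; BeginGameSpawn enables spawning once and clears the lost flag if the player pawn has lives left.
; SpawnWavesCounter counts spawns and stops at the wave cap; IncreaseMaxCount raises that cap, resets the count, advances the wave and compounds a difficulty multiplier.
; GameLost only prints a message, and the ready-check and walk-speed scaling logic is disconnected.
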(event `Begin Game Spawn`
  (if (not (`self.CanBeginGame`))
    (set `self.CanBeginGame` true)
    (set `self.CanSpawn` true)
    (bind _asbp_player_pawn (cast `/Game/Classes/Player/BP_PlayerPawn` (`GameplayStatics.GetPlayerPawn` 0)))
    (if (>= (`/Game/Classes/Player/BP_PlayerPawn.Lives` _asbp_player_pawn) 1)
      (bind _output_get (set `self.Game Lost` false))
      (`KismetSystemLibrary.PrintString` "Begin Game"))))

(event `Increase Max Count`
  (`KismetSystemLibrary.PrintString` "Call Increase" false)
  (set `self.MaxSpawnCount` (+ (`self.MaxSpawnCount`) 7))
  (set `self.CurrentSpawnCount` 0)
  (set `self.CanSpawn` true)
  (set `self.WaveCounter` (+ (`self.WaveCounter`) 1))
  (bind _output_get (set `self.DifficultyMultiplier` (* (`self.DifficultyMultiplier`) 1.03)))
  (`KismetSystemLibrary.PrintString` (`KismetStringLibrary.Conv_DoubleToString` _output_get)))

(event `self.ReceiveTick`
  (params (DeltaSeconds :type "Float (single-precision)")))

(fn `GameLost`
  (`KismetSystemLibrary.PrintString` "Game Lost")
  (return))

(fn `SpawnWavesCounter`
  (if (`self.CanSpawn`)
    (set `self.CurrentSpawnCount` (+ (`self.CurrentSpawnCount`) 1))
    (if (== (`self.CurrentSpawnCount`) (`self.MaxSpawnCount`))
      (set `self.CanSpawn` false))))

(fn `UserConstructionScript`)