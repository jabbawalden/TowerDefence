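; Enemy spawn point that registers with BP_GameModeMain and spawns three AI enemy types at its location in waves.
; Tick polls the game mode's spawn flags and spawns after a randomized Delay, choosing the type from WaveCounter and SpawnIndex through hard-coded switches for ten waves.
; Each spawn updates the game mode's counter.
; When spawning stops, a DoOnce waits SpawnWaitTime, then calls IncreaseMaxCount, re-arming once spawning resumes.
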(event `self.ReceiveBeginPlay`
  (bind _asbp_game_mode_main (cast `/Game/Classes/GameFiles/BP_GameModeMain` (`GameplayStatics.GetGameMode`)))
  (bind _returnvalue (`KismetArrayLibrary.Array_Add` (`/Game/Classes/GameFiles/BP_GameModeMain.SpawnArrays` _asbp_game_mode_main) self)))

(event `self.ReceiveTick`
  (params (DeltaSeconds :type "Float (single-precision)"))
  (bind _output_get (set `self.NewTime` (+ (`GameplayStatics.GetWorldDeltaSeconds`) (`self.TimeRate`))))
  (bind _asbp_game_mode_main (cast `/Game/Classes/GameFiles/BP_GameModeMain` (`GameplayStatics.GetGameMode`)))
  (if (`/Game/Classes/GameFiles/BP_GameModeMain.CanBeginGame` _asbp_game_mode_main)
    (bind _output_get_2 (set `self.Can Spawn` (`/Game/Classes/GameFiles/BP_GameModeMain.CanSpawn` _asbp_game_mode_main)))
    (if _output_get_2
      (`KismetSystemLibrary.Delay` _output_get)
      (`self.Spawn Enemy V2`)
      (goto _label :!via `Reset`)
      (else
        (`/Engine/EditorBlueprintResources/StandardMacros.DoOnce` false :!label _label
          (:`Completed`
            (`KismetSystemLibrary.Delay` (`self.SpawnWaitTime`))
            (`KismetSystemLibrary.PrintString` "ÅÖÄ----CAN SPAWN DELAY")
            (set `self.ReadyForNextWave` true)
            (bind _asbp_game_mode_main_2 (cast `/Game/Classes/GameFiles/BP_GameModeMain` (`GameplayStatics.GetGameMode`)))
            (`/Game/Classes/GameFiles/BP_GameModeMain.Increase Max Count` _asbp_game_mode_main_2)
            (set `self.ReadyForNextWave` false)))))))

(event `Spawn Enemy V2`
  (bind _spawnindex (`self.SpawnIndex`))
  (bind _spawnindex_2 (`self.SpawnIndex`))
  (bind _spawnindex_3 (`self.SpawnIndex`))
  (if (`self.Can Spawn`)
    (set `self.TimeRate` (`KismetMathLibrary.RandomFloatInRange` (`self.Min`) (`self.Max`)))
    (bind _asbp_game_mode_main (cast `/Game/Classes/GameFiles/BP_GameModeMain` (`GameplayStatics.GetGameMode`)))
    (switch `int` (`/Game/Classes/GameFiles/BP_GameModeMain.WaveCounter` _asbp_game_mode_main)
      (:`1`
        (`self.Spawn AI_One`))
      (:`2`
        (`self.Spawn AI_Two`))
      (:`3`
        (switch `int` _spawnindex_2
          (:`1`
            (`self.Spawn AI_One`))
          (:`2`
            (`self.Spawn AI_Two`))))
      (:`4`
        (switch `int` _spawnindex_2
          (:`1`
            (`self.Spawn AI_One` :!label _label_2))
          (:`2`
            (goto _label_2))
          (:`3`
            (goto _label_2))
          (:`4`
            (`self.Spawn AI_Two`))
          (:`5`
            (`self.Spawn AI_Three`))))
      (:`5`
        (switch `int` _spawnindex_2
          (:`1`
            (`self.Spawn AI_One` :!label _label_3))
          (:`2`
            (`self.Spawn AI_Two` :!label _label_4))
          (:`3`
            (goto _label_4))
          (:`4`
            (goto _label_3))))
      (:`6`
        (switch `int` (`self.SpawnIndex`)
          (:`1`
            (`self.Spawn AI_One`))
          (:`2`
            (`self.Spawn AI_Two` :!label _label_5))
          (:`3`
            (goto _label_5))
          (:`4`
            (goto _label_5))
          (:`5`
            (`self.Spawn AI_Three`))))
      (:`7`
        (switch `int` _spawnindex
          (:`1`
            (`self.Spawn AI_Two` :!label _label_6))
          (:`2`
            (goto _label_6))
          (:`3`
            (goto _label_6))
          (:`4`
            (`self.Spawn AI_Three` :!label _label_7))
          (:`5`
            (goto _label_7))))
      (:`8`
        (switch `int` _spawnindex
          (:`1`
            (`self.Spawn AI_One`))
          (:`2`
            (`self.Spawn AI_Two` :!label _label_8))
          (:`3`
            (goto _label_8))
          (:`4`
            (`self.Spawn AI_Three` :!label _label_9))
          (:`5`
            (goto _label_9))))
      (:`9`
        (switch `int` _spawnindex_3
          (:`1`
            (`self.Spawn AI_One` :!label _label_10))
          (:`2`
            (goto _label_10))
          (:`3`
            (goto _label_10))
          (:`4`
            (goto _label_10))
          (:`5`
            (goto _label_10))
          (:`6`
            (`self.Spawn AI_Two`))
          (:`7`
            (`self.Spawn AI_Three`))))
      (:`10`
        (switch `int` _spawnindex_3
          (:`1`
            (`self.Spawn AI_One` :!label _label_11))
          (:`2`
            (`self.Spawn AI_Two` :!label _label_12))
          (:`3`
            (goto _label_12))
          (:`4`
            (goto _label_12))
          (:`5`
            (`self.Spawn AI_Three` :!label _label_13))
          (:`6`
            (goto _label_13))
          (:`7`
            (goto _label_11)))))))

(fn `Spawn AI_One`
  (bind _returnvalue (`AIBlueprintHelperLibrary.SpawnAIFromClass` "/Game/Classes/AI/BP_AI_EnemyOne.BP_AI_EnemyOne_C" null (`self.K2_GetActorLocation`) (struct) true))
  (bind _asbp_game_mode_main (cast `/Game/Classes/GameFiles/BP_GameModeMain` (`GameplayStatics.GetGameMode`)))
  (`/Game/Classes/GameFiles/BP_GameModeMain.SpawnWavesCounter` _asbp_game_mode_main))

(fn `Spawn AI_Three`
  (`AIBlueprintHelperLibrary.SpawnAIFromClass` "/Game/Classes/AI/BP_AI_EnemyThree.BP_AI_EnemyThree_C" null (`self.K2_GetActorLocation`) (struct) true)
  (bind _asbp_game_mode_main (cast `/Game/Classes/GameFiles/BP_GameModeMain` (`GameplayStatics.GetGameMode`)))
  (`/Game/Classes/GameFiles/BP_GameModeMain.SpawnWavesCounter` _asbp_game_mode_main))

(fn `Spawn AI_Two`
  (`AIBlueprintHelperLibrary.SpawnAIFromClass` "/Game/Classes/AI/BP_AI_EnemyTwo.BP_AI_EnemyTwo_C" null (`self.K2_GetActorLocation`) (struct) true)
  (bind _asbp_game_mode_main (cast `/Game/Classes/GameFiles/BP_GameModeMain` (`GameplayStatics.GetGameMode`)))
  (`/Game/Classes/GameFiles/BP_GameModeMain.SpawnWavesCounter` _asbp_game_mode_main))

(fn `UserConstructionScript`)