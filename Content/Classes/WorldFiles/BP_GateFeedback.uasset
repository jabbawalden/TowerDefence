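; BP_GateFeedback is a visual countdown cue, apparently for a gate, built from a cube that stays hidden until triggered.
; GateFeedbackCountdown prints a debug string, reveals the cube, resets it to OriginalScale and plays the Shrink timeline from the start.
; Each timeline update subtracts a fixed step from world scale, so shrink speed depends on frame rate.
; When the timeline finishes, the cube hides without propagating to its children.
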(event `Gate Feedback Countdown`
  (bind _cube (`self.Cube`))
  (`KismetSystemLibrary.PrintString` "Call Feedback")
  (`SceneComponent.SetVisibility` (`self.Cube`) true true)
  (`SceneComponent.SetWorldScale3D` (`self.Cube`) (`self.OriginalScale`))
  (`Timeline|Shrink` :!via `PlayFromStart`
    (:`Update`
      (`SceneComponent.SetWorldScale3D` _cube (- (`SceneComponent.K2_GetComponentScale` _cube) (0.006 0.006 0.006))))
    (:`Finished`
      (`SceneComponent.SetVisibility` _cube false false))))

(event `self.ReceiveBeginPlay`
  (`SceneComponent.SetVisibility` (`self.Cube`) false false))

(fn `UserConstructionScript`)