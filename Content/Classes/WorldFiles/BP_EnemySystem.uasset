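; Enemy spawner that places AI checkpoints along its spline and spawns waves of enemies around its own location.
; BeginPlay spawns a SplinePointCheck actor at spline points in a counted loop.
; Tick polls BP_GameModeMain, spawning its chosen class on a delay at random XY offsets, passing itself via BPI_AISettings and updating the wave counter.
; When spawning closes, a DoOnce-gated delay raises the max count and checks wave status.
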(event `self.ReceiveBeginPlay`
  (bind _spline (`self.Spline`))
  (bind _currentspointcounter (`self.CurrentSPointCounter`))
  ;[0.321 0.6408 0.7302 1 35] Spawn Check Point For AI
  (set `self.MaxSPointCounter` (- (`SplineComponent.GetNumberOfSplinePoints` _spline) 1))
  (`|SpawnActorFromClass` "/Game/Classes/WorldFiles/SplinePointCheck.SplinePointCheck_C" (`KismetMathLibrary.Conv_VectorToTransform` (`SplineComponent.GetLocationAtSplinePoint` _spline (`self.CurrentSPointCounter`) "World")) "Undefined" "OverrideRootScale" null null :!label _label)
  (if (<= _currentspointcounter (`self.MaxSPointCounter`))
    (set `self.CurrentSPointCounter` (+ _currentspointcounter 1))
    (goto _label)))

(event `self.ReceiveTick`
  (params (DeltaSeconds :type "Float (single-precision)"))
  (bind _asbp_game_mode_main (cast `/Game/Classes/GameFiles/BP_GameModeMain` (`GameplayStatics.GetGameMode`)))
  (if (`/Game/Classes/GameFiles/BP_GameModeMain.CanBeginGame` _asbp_game_mode_main)
    (bind _output_get (set `self.CanSpawn` (`/Game/Classes/GameFiles/BP_GameModeMain.CanSpawn` _asbp_game_mode_main)))
    (if _output_get
      (bind _output_get_2 (set `self.NewTime` (+ (`GameplayStatics.GetWorldDeltaSeconds`) (`self.TimeRate`))))
      (`KismetSystemLibrary.Delay` _output_get_2)
      (`self.Spawn AI` (`/Game/Classes/GameFiles/BP_GameModeMain.ClassToSpawn` _asbp_game_mode_main))
      (else
        (`/Engine/EditorBlueprintResources/StandardMacros.DoOnce` false :!label _label_2
          (:`Completed`
            (`KismetSystemLibrary.Delay` (`self.SpawnWaitTime`))
            (`KismetSystemLibrary.PrintString` "ÅÖÄ----CAN SPAWN DELAY")
            (bind _asbp_game_mode_main_2 (cast `/Game/Classes/GameFiles/BP_GameModeMain` (`GameplayStatics.GetGameMode`)))
            (`/Game/Classes/GameFiles/BP_GameModeMain.IncreaseMaxCount` _asbp_game_mode_main_2)
            (`/Game/Classes/GameFiles/BP_GameModeMain.CheckWaveStatus` _asbp_game_mode_main_2)
            (goto _label_2 :!via `Reset`)))))))

(fn `Spawn AI`
  (params (EnemyClass :type "Pawn Class Reference"))
  (bind _returnvalue (`KismetMathLibrary.RandomFloatInRange` -70.0 70.0))
  (bind _returnvalue_2 (`AIBlueprintHelperLibrary.SpawnAIFromClass` EnemyClass null (+ (`KismetMathLibrary.MakeVector` _returnvalue _returnvalue) (`self.K2_GetActorLocation`))))
  (if (`KismetSystemLibrary.DoesImplementInterface` _returnvalue_2 "/Game/Classes/Buildings/Interfaces/BPI_AISettings.BPI_AISettings_C")
    (message `/Game/Classes/Buildings/Interfaces/BPI_AISettings.Set Enemy System Ref` _returnvalue_2 self)
    (bind _asbp_game_mode_main (cast `/Game/Classes/GameFiles/BP_GameModeMain` (`GameplayStatics.GetGameMode`)))
    (`/Game/Classes/GameFiles/BP_GameModeMain.SpawnWavesCounter` _asbp_game_mode_main)))

(fn `UserConstructionScript`)