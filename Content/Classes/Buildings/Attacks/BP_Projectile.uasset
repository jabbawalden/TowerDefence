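; Homing tower projectile that damages actors tagged Enemy.
; Each tick it turns toward TargetRunner while that is valid and moves forward at ProjectileSpeed, flying straight once the target is gone.
; Its sphere overlap deals base, pierce and blunt damage to enemies, plus optional virus damage at a set rate sent by message.
; Any sphere overlap, enemy or not, destroys the projectile.
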(event `self.ReceiveTick`
  (params (DeltaSeconds :type "Float (single-precision)"))
  (bind _targetrunner (`self.TargetRunner`))
  (`/Engine/EditorBlueprintResources/StandardMacros.IsValid` _targetrunner
    (:`Is Valid`
      (`self.K2_SetActorRotation` (`KismetMathLibrary.FindLookAtRotation` (`self.K2_GetActorLocation`) (`self.K2_GetActorLocation` _targetrunner))))
    (:`Is Not Valid`
      _))
  (`self.K2_SetActorLocation` (+ (* (`self.GetActorForwardVector`) (* (`self.ProjectileSpeed`) (`GameplayStatics.GetWorldDeltaSeconds`))) (`self.K2_GetActorLocation`))))

(event `self.Sphere.OnComponentBeginOverlap`
  (params (OverlappedComponent :type "PrimitiveComponent Object Reference") (OtherActor :type "Actor Object Reference") (OtherComp :type "PrimitiveComponent Object Reference") (OtherBodyIndex :type Integer) (bFromSweep :type Boolean) (SweepResult :type "HitResult Structure (by ref)"))
  (if (`self.ActorHasTag` OtherActor "Enemy")
    (`/Game/Classes/GameFiles/BP_FunctionLibrary.Deal Damage To Actor` OtherActor (`self.BaseDamage`) (`self.Pierce Damage`) (`self.Blunt Damage`))
    (`/Engine/EditorBlueprintResources/StandardMacros.IsValid` OtherActor
      (:`Is Valid`
        (if (`self.CanInflictVirusDamage`)
          (message `/Game/Classes/AI/BPI_AoeEffects.AI Virus Damage` OtherActor (`self.VirusDamage`) (`self.VirusDamageRate`))))
      (:`Is Not Valid`
        _))
    (`self.K2_DestroyActor` :!label _label)
    (elif true
      (goto _label))))

(fn `UserConstructionScript`)