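; Mortar shell actor that lobs toward a target runner and spawns an area-of-effect impact where it lands.
; On BeginPlay it applies an upward force to its Sphere and rotates once to face the target's location, with no later homing.
; Tick advances only X and Y along the forward vector, leaving height to physics for the arc.
; Overlapping an Enemy or Ground tagged actor spawns BP_MortarImpactAOE with its damage settings, then destroys the shell.
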(event `self.ReceiveBeginPlay`
  (bind _targetrunner (`self.TargetRunner`))
  (`/Engine/EditorBlueprintResources/StandardMacros.IsValid` _targetrunner
    (:`Is Valid`
      (`PrimitiveComponent.AddForce` (`self.Sphere`) (`KismetMathLibrary.MakeVector` 0.0 0.0 (`self.UpwardForce`)) "None" false)
      (`self.K2_SetActorRotation` (`KismetMathLibrary.FindLookAtRotation` (`self.K2_GetActorLocation`) (`self.K2_GetActorLocation` _targetrunner))))))

(event `self.ReceiveTick`
  (params (DeltaSeconds :type "Float (single-precision)"))
  (bind (_returnvalue_x _returnvalue_y _returnvalue_z) (`KismetMathLibrary.BreakVector` (`self.K2_GetActorLocation`)))
  (bind (_returnvalue_x_2 _returnvalue_y_2) (`KismetMathLibrary.BreakVector` (+ (* (`self.GetActorForwardVector`) (* (`self.ProjectileSpeed`) (`GameplayStatics.GetWorldDeltaSeconds`))) (`self.K2_GetActorLocation`))))
  (`self.K2_SetActorLocation` (`KismetMathLibrary.MakeVector` _returnvalue_x_2 _returnvalue_y_2 _returnvalue_z)))

(event `self.Sphere.OnComponentBeginOverlap`
  (params (OverlappedComponent :type "PrimitiveComponent Object Reference") (OtherActor :type "Actor Object Reference") (OtherComp :type "PrimitiveComponent Object Reference") (OtherBodyIndex :type Integer) (bFromSweep :type Boolean) (SweepResult :type "HitResult Structure (by ref)"))
  (if (or (`self.ActorHasTag` OtherActor "Enemy") (`self.ActorHasTag` OtherActor "Ground"))
    (`|SpawnActorFromClass` "/Game/Classes/Buildings/Attacks/BP_MortarImpactAOE.BP_MortarImpactAOE_C" (`SceneComponent.K2_GetComponentToWorld` (`self.Sphere`)) "Undefined" "OverrideRootScale" null (`self.BaseDamage`) (`self.PierceDamage`) (`self.BluntDamage`) (`self.VirusDamage`) (`self.VirusDamageRate`) (`self.CanInflictVirusDamage`) null)
    (`self.K2_DestroyActor`)))

(fn `UserConstructionScript`)