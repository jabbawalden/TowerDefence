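; Mortar impact area-of-effect actor that damages enemies at the shell's landing point.
; On BeginPlay it spawns a scaled explosion emitter and destroys itself after a brief delay.
; During that window, sphere overlaps with Enemy-tagged actors deal base, pierce and blunt damage, and optionally send a virus damage-over-time message.
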(event `self.Sphere.OnComponentBeginOverlap`
  (params (OverlappedComponent :type "PrimitiveComponent Object Reference") (OtherActor :type "Actor Object Reference") (OtherComp :type "PrimitiveComponent Object Reference") (OtherBodyIndex :type Integer) (bFromSweep :type Boolean) (SweepResult :type "HitResult Structure (by ref)"))
  (`/Engine/EditorBlueprintResources/StandardMacros.IsValid` OtherActor
    (:`Is Valid`
      (if (`self.ActorHasTag` OtherActor "Enemy")
        (`/Game/Classes/GameFiles/BP_FunctionLibrary.Deal Damage To Actor` OtherActor (`self.BaseDamage`) (`self.Pierce Damage`) (`self.Blunt Damage`))
        (if (`self.CanInflictVirusDamage`)
          (`/Engine/EditorBlueprintResources/StandardMacros.IsValid` OtherActor
            (:`Is Valid`
              (message `/Game/Classes/AI/BPI_AoeEffects.AI Virus Damage` OtherActor (`self.VirusDamage`) (`self.VirusDamageRate`)))))))))

(event `self.ReceiveBeginPlay`
  (`GameplayStatics.SpawnEmitterAtLocation` "/Game/StarterContent/Particles/P_Explosion.P_Explosion" (`self.K2_GetActorLocation`) (struct) (2.5 2.5 2.5))
  (`KismetSystemLibrary.Delay` 0.1)
  (`self.K2_DestroyActor`))

(fn `UserConstructionScript`)