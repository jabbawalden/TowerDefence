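; BP_EnergyPlant is a power building that shares its EnergyCapacity among registered structures.
; Actors entering EnergyRange that implement BPI_StructureStatus receive a reference to the plant, and AddEnergyStructureArray registers structures.
; EnergyPlantEnergyInitiate adds an equal share of capacity to each structure's CBP_EnergyComponent EnergyAddAmount, accumulating on repeat calls.
; ReInitializeEnergy is an empty stub.
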(event `self.EnergyRange.OnComponentBeginOverlap`
  (params (OverlappedComponent :type "PrimitiveComponent Object Reference") (OtherActor :type "Actor Object Reference") (OtherComp :type "PrimitiveComponent Object Reference") (OtherBodyIndex :type Integer) (bFromSweep :type Boolean) (SweepResult :type "HitResult Structure (by ref)"))
  (`self.CheckForStructure` OtherActor))

(event `/Game/Classes/Buildings/Interfaces/BPI_StructureStatus.EnergyPlantEnergyInitiate`
  (`self.SetEnergyAddAmounts`))

(event `/Game/Classes/Buildings/Interfaces/BPI_StructureStatus.AddEnergyStructureArray`
  (params (Actor :type "Actor Object Reference"))
  (`/Engine/EditorBlueprintResources/StandardMacros.IsValid` Actor
    (:`Is Valid`
      (`KismetArrayLibrary.Array_Add` (`self.StructureArray`) Actor))))

(fn `CheckForStructure`
  (params (ActorCheck :type "Actor Object Reference"))
  (`/Engine/EditorBlueprintResources/StandardMacros.IsValid` ActorCheck
    (:`Is Valid`
      (if (`KismetSystemLibrary.DoesImplementInterface` ActorCheck "/Game/Classes/Buildings/Interfaces/BPI_StructureStatus.BPI_StructureStatus_C")
        (message `/Game/Classes/Buildings/Interfaces/BPI_StructureStatus.SetEnergyPlantReference` ActorCheck self)))))

(fn `ReInitializeEnergy`)

(fn `SetEnergyAddAmounts`
  (for _array_element (`self.StructureArray`)
    (bind _returnvalue (`self.GetComponentByClass` _array_element "/Game/Classes/Components/CBP_EnergyComponent.CBP_EnergyComponent_C"))
    (`/Engine/EditorBlueprintResources/StandardMacros.IsValid` _returnvalue
      (:`Is Valid`
        (set `/Game/Classes/Components/CBP_EnergyComponent.EnergyAddAmount` (+ (`/Game/Classes/Components/CBP_EnergyComponent.EnergyAddAmount` _returnvalue) (/ (`self.EnergyCapacity`) (`KismetMathLibrary.Conv_IntToDouble` (`KismetArrayLibrary.Array_Length` (`self.StructureArray`))))) _returnvalue)))))

(fn `UserConstructionScript`)