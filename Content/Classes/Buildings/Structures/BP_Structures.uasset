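; Building structure actor that shows a ghost preview and checks whether its placement is valid.
; Until built, each Tick traces down from four origin points for actors tagged RaisedGround, updating each result only on a hit.
; All four must pass to turn the ghost green and set ValidBuild; otherwise it turns red.
; ScaleTriggerToSize collapses sphere or cube triggers to zero scale, then restores unit scale after a short delay.
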(event `self.ReceiveBeginPlay`
  (set `self.CanAttack` false)
  (`KismetSystemLibrary.PrintString` "Call begin play")
  (`SceneComponent.SetVisibility` (`self.GhostStructure`) true false)
  (set `self.AmBuilt` false))

(event `self.ReceiveTick`
  (params (DeltaSeconds :type "Float (single-precision)"))
  (if (not (`self.AmBuilt`))
    (`self.LineTrace`)))

(event `ResetScale`
  (bind _triggersphere (`self.TriggerSphere`))
  (bind _triggercube (`self.TriggerCube`))
  (`KismetSystemLibrary.Delay` 0.1)
  (`|ExecutionSequence`
    (:`then_0`
      (`/Engine/EditorBlueprintResources/StandardMacros.IsValid` _triggersphere
        (:`Is Valid`
          (`SceneComponent.SetWorldScale3D` _triggersphere (1.0 1.0 1.0)))))
    (:`then_1`
      (`/Engine/EditorBlueprintResources/StandardMacros.IsValid` _triggercube
        (:`Is Valid`
          (`SceneComponent.SetWorldScale3D` _triggercube (1.0 1.0 1.0)))))))

(fn `LineTrace`
  (bind _returnvalue (`SceneComponent.K2_GetComponentLocation` (`self.LTOrigin4`)))
  (bind _returnvalue_2 (`SceneComponent.K2_GetComponentLocation` (`self.LTOrigin1`)))
  (bind _returnvalue_3 (`SceneComponent.K2_GetComponentLocation` (`self.LTOrigin2`)))
  (bind _returnvalue_4 (`SceneComponent.K2_GetComponentLocation` (`self.LTOrigin3`)))
  (`|ExecutionSequence`
    (:`then_0`
      (bind (_outhit _returnvalue_5) (`KismetSystemLibrary.LineTraceSingle` _returnvalue_2 (+ _returnvalue_2 (0.0 0.0 -200.0)) "TraceTypeQuery1"))
      (if _returnvalue_5
        (set `self.LT1` (`self.ActorHasTag` (`.HitActor` (`GameplayStatics.BreakHitResult` _outhit)) "RaisedGround"))))
    (:`then_1`
      (bind (_outhit_2 _returnvalue_6) (`KismetSystemLibrary.LineTraceSingle` _returnvalue_3 (+ _returnvalue_3 (0.0 0.0 -200.0)) "TraceTypeQuery1"))
      (if _returnvalue_6
        (set `self.LT2` (`self.ActorHasTag` (`.HitActor` (`GameplayStatics.BreakHitResult` _outhit_2)) "RaisedGround"))))
    (:`then_2`
      (bind (_outhit_3 _returnvalue_7) (`KismetSystemLibrary.LineTraceSingle` _returnvalue_4 (+ _returnvalue_4 (0.0 0.0 -200.0)) "TraceTypeQuery1"))
      (if _returnvalue_7
        (set `self.LT3` (`self.ActorHasTag` (`.HitActor` (`GameplayStatics.BreakHitResult` _outhit_3)) "RaisedGround"))))
    (:`then_3`
      (bind (_outhit_4 _returnvalue_8) (`KismetSystemLibrary.LineTraceSingle` _returnvalue (+ _returnvalue (0.0 0.0 -200.0)) "TraceTypeQuery1"))
      (if _returnvalue_8
        (set `self.LT4` (`self.ActorHasTag` (`.HitActor` (`GameplayStatics.BreakHitResult` _outhit_4)) "RaisedGround"))))
    (:`then_4`
      (if (`self.LT1`)
        (if (`self.LT2`)
          (if (`self.LT3`)
            (if (`self.LT4`)
              (`self.SetGhostGreen`)
              (else
                (`self.SetGhostRed` :!label _label)))
            (else
              (goto _label)))
          (else
            (goto _label)))
        (else
          (goto _label))))))

(fn `ScaleTriggerToSize`
  (params (TriggerSphere :type "SphereComponent Object Reference") (TriggerCube :type "BoxComponent Object Reference"))
  (`|ExecutionSequence`
    (:`then_0`
      (`/Engine/EditorBlueprintResources/StandardMacros.IsValid` TriggerSphere
        (:`Is Valid`
          (bind _output_get (set `self.TriggerSphere` TriggerSphere))
          (`SceneComponent.SetWorldScale3D` _output_get (0.0 0.0 0.0)))))
    (:`then_1`
      (`/Engine/EditorBlueprintResources/StandardMacros.IsValid` TriggerCube
        (:`Is Valid`
          (bind _output_get_2 (set `self.TriggerCube` TriggerCube))
          (`SceneComponent.SetWorldScale3D` _output_get_2 (0.0 0.0 0.0))))))
  (`self.ResetScale`))

(fn `SetGhostGreen`
  (bind _ghoststructure (`self.GhostStructure`))
  (for _index (range (+ (`PrimitiveComponent.GetNumMaterials` _ghoststructure) 1))
    (`PrimitiveComponent.SetMaterial` _ghoststructure _index "/Game/Classes/Materials/M_StructureGhostGreen.M_StructureGhostGreen")
    (set `self.ValidBuild` true)))

(fn `SetGhostRed`
  (bind _ghoststructure (`self.GhostStructure`))
  (for _index (range (+ (`PrimitiveComponent.GetNumMaterials` _ghoststructure) 1))
    (`PrimitiveComponent.SetMaterial` _ghoststructure _index "/Game/Classes/Materials/M_StructureGhostRed.M_StructureGhostRed")
    (set `self.ValidBuild` false)))

(fn `UserConstructionScript`)