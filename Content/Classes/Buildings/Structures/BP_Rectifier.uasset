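; BP_Rectifier is a buildable area-effect structure that slows enemies and can be upgraded to weaken or infect them.
; Once built, it reveals its mesh, sizes its trigger and notifies linked energy plants.
; Overlaps apply or clear effects through BPI_AoeEffects, using an afflicted counter on enemies to handle overlapping sources.
; Paid, capped blunt, pierce and virus upgrades unlock effects, with diminishing resistance-reduction increments pushed to tracked enemies.
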(event `self.ReceiveTick`
  (params (DeltaSeconds :type "Float (single-precision)"))
  (`parent.ReceiveTick` 0.0))

(event `self.ReceiveBeginPlay`
  (`parent.ReceiveBeginPlay`)
  (`SceneComponent.SetVisibility` (`self.BluntDmg`) false false)
  (`SceneComponent.SetVisibility` (`self.PierceDmg`) false false)
  (`SceneComponent.SetVisibility` (`self.VirusDmg`) false false)
  (`SceneComponent.SetVisibility` (`self.MainBuilding`) false false))

(event `/Game/Classes/Buildings/Interfaces/BPI_StructureStatus.StructureBuilt`
  (set `self.CanAttack` true)
  (`SceneComponent.SetVisibility` (`self.GhostStructure`) false false)
  (`SceneComponent.SetVisibility` (`self.MainBuilding`) true false)
  (`self.ScaleTriggerToSize` null (`self.AreaEffect`))
  (set `self.AmBuilt` true)
  (for _array_element (`self.EnergyPlantRef`)
    (bind _asbp_energy_plant (cast `/Game/Classes/Buildings/Structures/BP_EnergyPlant` _array_element))
    (`self.StructureEnergyInitiate` _asbp_energy_plant)))

(event `self.AreaEffect.OnComponentBeginOverlap`
  (params (OverlappedComponent :type "PrimitiveComponent Object Reference") (OtherActor :type "Actor Object Reference") (OtherComp :type "PrimitiveComponent Object Reference") (OtherBodyIndex :type Integer) (bFromSweep :type Boolean) (SweepResult :type "HitResult Structure (by ref)"))
  (`self.AddRemoveEnemy` true OtherActor))

(event `/Game/Classes/AI/BPI_ModifierBehaviour.Increase Blunt Damage`
  ;[1 0.9205 0.3716] Add functionality for giving these effects to enemies within an array
  (if (>= (`self.BluntUpgradeCount`) (`self.BluntUpgradeMaxCount`))
    (`KismetSystemLibrary.PrintString` "Max Blunt")
    (else
      (if (`self.CanLowerBluntResistance`)
        (`self.Increase Blunt Deduction`)
        (`self.Blunt Resistance Adjust`)
        (else
          (set `self.CanLowerBluntResistance` true)
          (`SceneComponent.SetVisibility` (`self.BluntDmg`) true true)))
      (`/Game/Classes/Player/BP_PlayerPawn.ResourceDeduction` (`self.PlayerPawn`) (`/Game/Classes/GameFiles/BP_GameModeMain.BluntModCost` (`self.GameMode`)))
      (set `self.BluntUpgradeCount` (+ (`self.BluntUpgradeCount`) 1)))))

(event `self.AreaEffect.OnComponentEndOverlap`
  (params (OverlappedComponent :type "PrimitiveComponent Object Reference") (OtherActor :type "Actor Object Reference") (OtherComp :type "PrimitiveComponent Object Reference") (OtherBodyIndex :type Integer))
  (`self.AddRemoveEnemy` false OtherActor))

(event `/Game/Classes/AI/BPI_ModifierBehaviour.Increase Pierce Damage`
  ;[1 0.9205 0.3716] Add functionality for giving these effects to enemies within an array
  (if (>= (`self.PierceUpgradeCount`) (`self.PierceUpgradeMaxCount`))
    (`KismetSystemLibrary.PrintString` "Max Pierce")
    (else
      (if (`self.CanLowerPierceResistance`)
        (`self.Increase Pierce Deduction`)
        (`self.Pierce Resistance Adjust`)
        (else
          (set `self.CanLowerPierceResistance` true)
          (`SceneComponent.SetVisibility` (`self.PierceDmg`) true true)))
      (`/Game/Classes/Player/BP_PlayerPawn.ResourceDeduction` (`self.PlayerPawn`) (`/Game/Classes/GameFiles/BP_GameModeMain.PierceModCost` (`self.GameMode`)))
      (set `self.PierceUpgradeCount` (+ (`self.PierceUpgradeCount`) 1)))))

(event `/Game/Classes/AI/BPI_ModifierBehaviour.Increase Base Damage`
  ;[1 0.9205 0.3716] Add functionality for giving these effects to enemies within an array
)

(event `/Game/Classes/AI/BPI_ModifierBehaviour.Add Virus Damage`
  (bind _playerpawn (`self.PlayerPawn`))
  (bind _virusmodcost (`/Game/Classes/GameFiles/BP_GameModeMain.VirusModCost` (`self.GameMode`)))
  ;[1 0.9205 0.3716] Add functionality for giving these effects to enemies within an array
  (if (>= (`self.VirusUpgradeCount`) (`self.VirusUpgradeMaxCount`))
    (`KismetSystemLibrary.PrintString` "Max Virus")
    (else
      (if (`self.CanInflictVirusDamage`)
        (`self.Increase Virus Attack Rate`)
        (`self.Virus Attack Rate Adjust`)
        (`/Game/Classes/Player/BP_PlayerPawn.ResourceDeduction` _playerpawn _virusmodcost)
        (else
          (set `self.CanInflictVirusDamage` true)
          (`SceneComponent.SetVisibility` (`self.VirusDmg`) true true)
          (`/Game/Classes/Player/BP_PlayerPawn.ResourceDeduction` _playerpawn _virusmodcost)))
      (set `self.VirusUpgradeCount` (+ (`self.VirusUpgradeCount`) 1))
      (for _array_element (`self.EnemyArray`)
        (if (`self.CanInflictVirusDamage`)
          (`/Engine/EditorBlueprintResources/StandardMacros.IsValid` _array_element
            (:`Is Valid`
              (message `/Game/Classes/AI/BPI_AoeEffects.AI Virus Damage` _array_element (`self.VirusDamage`) (`self.VirusDamageRate`)))))))))

(fn `AddRemoveEnemy`
  (params (InRange :type Boolean) (Actor :type "Actor Object Reference"))
  (`/Engine/EditorBlueprintResources/StandardMacros.IsValid` Actor
    (:`Is Valid`
      (if (`KismetSystemLibrary.DoesImplementInterface` Actor "/Game/Classes/AI/BPI_AoeEffects.BPI_AoeEffects_C")
        (if InRange
          (bind (_isafflicted _canvirusdamage) (`/Game/Classes/GameFiles/BP_FunctionLibrary.CheckIfAfflicted` Actor))
          (if _isafflicted
            (message `/Game/Classes/AI/BPI_AoeEffects.AI ADD Afflicted Counter` Actor)
            (if (not _canvirusdamage)
              (if (`self.CanInflictVirusDamage`) :!label _label
                (message `/Game/Classes/AI/BPI_AoeEffects.AI Virus Damage` Actor (`self.VirusDamage`) (`self.VirusDamageRate`))))
            (else
              (message `/Game/Classes/AI/BPI_AoeEffects.AI ADD Afflicted Counter` Actor)
              (if (`self.CanAttack`)
                (message `/Game/Classes/AI/BPI_AoeEffects.AI Slow Down` Actor (`self.Slow down severity`))
                (`KismetArrayLibrary.Array_Add` (`self.EnemyArray`) Actor)
                (`|ExecutionSequence`
                  (:`then_0`
                    (goto _label))
                  (:`then_1`
                    (if (`self.CanLowerPierceResistance`)
                      (message `/Game/Classes/AI/BPI_AoeEffects.AI Reduce Pierce Resistance` Actor true (- (`self.PercentCheck`) (`self.LowerPierceResistance`)))))
                  (:`then_2`
                    (if (`self.CanLowerBluntResistance`)
                      (message `/Game/Classes/AI/BPI_AoeEffects.AI Reduce Blunt Resistance` Actor true (- (`self.PercentCheck`) (`self.LowerBluntResistance`)))))))))
          (else
            (message `/Game/Classes/AI/BPI_AoeEffects.AI SUB Afflicted Counter` Actor)
            (bind _isafflicted_2 (`/Game/Classes/GameFiles/BP_FunctionLibrary.CheckIfAfflicted` Actor))
            (if (not _isafflicted_2)
              (message `/Game/Classes/AI/BPI_AoeEffects.AI Resume Speed` Actor)
              (if (`self.CanInflictVirusDamage`)
                (`KismetArrayLibrary.Array_RemoveItem` (`self.EnemyArray`) Actor)
                (`|ExecutionSequence`
                  (:`then_0`
                    (if (`self.CanInflictVirusDamage`)
                      (message `/Game/Classes/AI/BPI_AoeEffects.AI Virus Damage Stop` Actor)))
                  (:`then_1`
                    (if (`self.CanLowerPierceResistance`)
                      (message `/Game/Classes/AI/BPI_AoeEffects.AI Reduce Pierce Resistance` Actor true 0.0)))
                  (:`then_2`
                    (if (`self.CanLowerBluntResistance`)
                      (message `/Game/Classes/AI/BPI_AoeEffects.AI Reduce Blunt Resistance` Actor true 0.0))))))))))))

(fn `Blunt Resistance Adjust`
  (if (`self.CanLowerBluntResistance`)
    (for _array_element (`self.EnemyArray`)
      (message `/Game/Classes/AI/BPI_AoeEffects.AI Reduce Blunt Resistance` _array_element true (- (`self.PercentCheck`) (`self.LowerBluntResistance`))))))

(fn `Increase Blunt Deduction`
  (bind _lowerbluntresistance (`self.LowerBluntResistance`))
  (bind _output_get (set `self.LowerBluntResistance` (+ _lowerbluntresistance (* _lowerbluntresistance (`self.BluntAdd`)))))
  (set `self.BluntAdd` (* (`self.BluntAdd`) 0.65))
  (`KismetSystemLibrary.PrintString` (`KismetStringLibrary.Conv_DoubleToString` _output_get)))

(fn `Increase Pierce Deduction`
  (bind _output_get (set `self.LowerPierceResistance` (+ (`self.LowerPierceResistance`) (* (`self.LowerPierceResistance`) (`self.PierceAdd`)))))
  (set `self.PierceAdd` (* (`self.PierceAdd`) 0.65))
  (`KismetSystemLibrary.PrintString` (`KismetStringLibrary.Conv_DoubleToString` _output_get)))

(fn `Increase Virus Attack Rate`
  (set `self.VirusDecrease` (- (`self.VirusDamageRate`) (`self.VirusDecrease`))))

(fn `Pierce Resistance Adjust`
  (if (`self.CanLowerPierceResistance`)
    (for _array_element (`self.EnemyArray`)
      (message `/Game/Classes/AI/BPI_AoeEffects.AI Reduce Pierce Resistance` _array_element true (- (`self.PercentCheck`) (`self.LowerPierceResistance`))))))

(fn `UserConstructionScript`)

(fn `Virus Attack Rate Adjust`
  (if (`self.CanInflictVirusDamage`)
    (for _array_element (`self.EnemyArray`)
      (message `/Game/Classes/AI/BPI_AoeEffects.AI Virus Damage` _array_element 0.0 (`self.VirusDamageRate`)))))