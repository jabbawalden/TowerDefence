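; BP_B_Gunner_Ghost is a gunner tower that automatically shoots projectiles at enemies within its range.
; A range trigger maintains an array of Enemy-tagged actors, and Tick fires at the first entry's target component on a fire-rate timer.
; Each BP_Projectile receives the tower's damage stats and owner.
; Upgrade events raise base, blunt or pierce damage or enable virus damage, with blunt, pierce and virus upgrades revealing hidden indicator components.
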(event `self.ReceiveBeginPlay`
  (`SceneComponent.SetVisibility` (`self.BluntDmg`) false false)
  (`SceneComponent.SetVisibility` (`self.PierceDmg`) false false)
  (`SceneComponent.SetVisibility` (`self.VirusDmg`) false false))

(event `self.ReceiveTick`
  (params (DeltaSeconds :type "Float (single-precision)"))
  (bind _output (`|GetArrayItem` (`self.EnemyArray`)))
  (if (> (`KismetArrayLibrary.Array_Length` (`self.EnemyArray`)) 0)
    (if (>= (`KismetSystemLibrary.GetGameTimeInSeconds`) (`self.NewTime`))
      (`self.Shoot Projectile` _output (`SceneComponent.K2_GetComponentLocation` (`self.GetComponentByClass` _output "/Game/Classes/Components/TargetComponentV2.TargetComponentV2_C")))
      (set `self.NewTime` (+ (`KismetSystemLibrary.GetGameTimeInSeconds`) (`self.FireRate`))))))

(event `/Game/Classes/AI/BPI_ModifierBehaviour.Increase Blunt Damage`
  (set `self.BluntDamage` (+ (`self.BluntDamage`) 60.0))
  (`SceneComponent.SetVisibility` (`self.BluntDmg`) true true))

(event `/Game/Classes/AI/BPI_ModifierBehaviour.Increase Pierce Damage`
  (set `self.PierceDamage` (+ (`self.PierceDamage`) 60.0))
  (`SceneComponent.SetVisibility` (`self.PierceDmg`) true true))

(event `self.TowerRangeTrigger.OnComponentBeginOverlap`
  (params (OverlappedComponent :type "PrimitiveComponent Object Reference") (OtherActor :type "Actor Object Reference") (OtherComp :type "PrimitiveComponent Object Reference") (OtherBodyIndex :type Integer) (bFromSweep :type Boolean) (SweepResult :type "HitResult Structure (by ref)"))
  (`/Engine/EditorBlueprintResources/StandardMacros.IsValid` OtherActor
    (:`Is Valid`
      (if (`self.ActorHasTag` OtherActor "Enemy")
        (`KismetArrayLibrary.Array_Add` (`self.EnemyArray`) OtherActor)))))

(event `/Game/Classes/AI/BPI_ModifierBehaviour.Increase Base Damage`
  (set `self.BaseDamage` (+ (`self.BaseDamage`) 10.0)))

(event `/Game/Classes/AI/BPI_ModifierBehaviour.Add Virus Damage`
  (set `self.CanInflictVirusDamage` true)
  (`SceneComponent.SetVisibility` (`self.VirusDmg`) true true))

(event `self.TowerRangeTrigger.OnComponentEndOverlap`
  (params (OverlappedComponent :type "PrimitiveComponent Object Reference") (OtherActor :type "Actor Object Reference") (OtherComp :type "PrimitiveComponent Object Reference") (OtherBodyIndex :type Integer))
  (`/Engine/EditorBlueprintResources/StandardMacros.IsValid` OtherActor
    (:`Is Valid`
      (if (`self.ActorHasTag` OtherActor "Enemy")
        (`KismetArrayLibrary.Array_RemoveItem` (`self.EnemyArray`) OtherActor)))))

(fn `Shoot Projectile`
  (params (ProjectileTarget :type "Actor Object Reference") (TargetLocation :type "Vector Structure"))
  (`|SpawnActorFromClass` "/Game/Classes/Buildings/Attacks/BP_Projectile.BP_Projectile_C" (`KismetMathLibrary.MakeTransform` (`SceneComponent.K2_GetComponentLocation` (`self.ShotOrigin`))) "Undefined" "OverrideRootScale" null ProjectileTarget (`self.BaseDamage`) (`self.PierceDamage`) (`self.BluntDamage`) (`self.VirusDamage`) (`self.CanInflictVirusDamage`) (`self.VirusDamageRate`) TargetLocation self null))

(fn `UserConstructionScript`)