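; Rectifier ghost structure with an area effect that slows and debuffs overlapping actors implementing BPI_AoeEffects.
; An afflicted check and per-actor counter keep effects from stacking across overlaps.
; Upgrade events unlock virus damage and lower pierce or blunt resistance, showing matching components; only virus damage reaches actors already in range.
; On exit, speed resumes, but list removal and resistance resets run only with virus damage unlocked.
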(event `self.ReceiveBeginPlay`
  (`SceneComponent.SetVisibility` (`self.BluntDmg`) false false)
  (`SceneComponent.SetVisibility` (`self.PierceDmg`) false false)
  (`SceneComponent.SetVisibility` (`self.VirusDmg`) false false))

(event `self.AreaEffect.OnComponentBeginOverlap`
  (params (OverlappedComponent :type "PrimitiveComponent Object Reference") (OtherActor :type "Actor Object Reference") (OtherComp :type "PrimitiveComponent Object Reference") (OtherBodyIndex :type Integer) (bFromSweep :type Boolean) (SweepResult :type "HitResult Structure (by ref)"))
  (if (`KismetSystemLibrary.DoesImplementInterface` OtherActor "/Game/Classes/AI/BPI_AoeEffects.BPI_AoeEffects_C")
    (bind _isafflicted (`/Game/Classes/GameFiles/BP_FunctionLibrary.CheckIfAfflicted` OtherActor))
    (if _isafflicted
      (message `/Game/Classes/AI/BPI_AoeEffects.AI ADD Afflicted Counter` OtherActor)
      (else
        (message `/Game/Classes/AI/BPI_AoeEffects.AI ADD Afflicted Counter` OtherActor)
        (message `/Game/Classes/AI/BPI_AoeEffects.AI Slow Down` OtherActor (`self.Slow down severity`))
        (`KismetArrayLibrary.Array_Add` (`self.EnemiesInRange`) OtherActor)
        (`|ExecutionSequence`
          (:`then_0`
            (if (`self.CanInflictVirusDamage`)
              (message `/Game/Classes/AI/BPI_AoeEffects.AI Virus Damage` OtherActor (`self.VirusDamage`) (`self.VirusDamageRate`))))
          (:`then_1`
            (if (`self.CanLowerPierceResistance`)
              (message `/Game/Classes/AI/BPI_AoeEffects.AI Reduce Pierce Resistance` OtherActor true (- (`self.PercentCheck`) (`self.LowerPierceResistance`)))))
          (:`then_2`
            (if (`self.CanLowerBluntResistance`)
              (message `/Game/Classes/AI/BPI_AoeEffects.AI Reduce Blunt Resistance` OtherActor true (- (`self.PercentCheck`) (`self.LowerBluntResistance`))))))))))

(event `self.AreaEffect.OnComponentEndOverlap`
  (params (OverlappedComponent :type "PrimitiveComponent Object Reference") (OtherActor :type "Actor Object Reference") (OtherComp :type "PrimitiveComponent Object Reference") (OtherBodyIndex :type Integer))
  (if (`KismetSystemLibrary.DoesImplementInterface` OtherActor "/Game/Classes/AI/BPI_AoeEffects.BPI_AoeEffects_C")
    (message `/Game/Classes/AI/BPI_AoeEffects.AI SUB Afflicted Counter` OtherActor)
    (bind _isafflicted (`/Game/Classes/GameFiles/BP_FunctionLibrary.CheckIfAfflicted` OtherActor))
    (if (not _isafflicted)
      (message `/Game/Classes/AI/BPI_AoeEffects.AI Resume Speed` OtherActor)
      (if (`self.CanInflictVirusDamage`)
        (`KismetArrayLibrary.Array_RemoveItem` (`self.EnemiesInRange`) OtherActor)
        (`|ExecutionSequence`
          (:`then_0`
            (if (`self.CanInflictVirusDamage`)
              (message `/Game/Classes/AI/BPI_AoeEffects.AI Virus Damage Stop` OtherActor)))
          (:`then_1`
            (if (`self.CanLowerPierceResistance`)
              (message `/Game/Classes/AI/BPI_AoeEffects.AI Reduce Pierce Resistance` OtherActor true 0.0)))
          (:`then_2`
            (if (`self.CanLowerBluntResistance`)
              (message `/Game/Classes/AI/BPI_AoeEffects.AI Reduce Blunt Resistance` OtherActor true 0.0))))))))

(event `/Game/Classes/AI/BPI_ModifierBehaviour.Increase Blunt Damage`
  ;[1 0.9205 0.3716] Add functionality for giving these effects to enemies within an array
  (set `self.CanLowerBluntResistance` true)
  (`SceneComponent.SetVisibility` (`self.BluntDmg`) true true))

(event `/Game/Classes/AI/BPI_ModifierBehaviour.Increase Pierce Damage`
  ;[1 0.9205 0.3716] Add functionality for giving these effects to enemies within an array
  (set `self.CanLowerPierceResistance` true)
  (`SceneComponent.SetVisibility` (`self.PierceDmg`) true true))

(event `/Game/Classes/AI/BPI_ModifierBehaviour.Increase Base Damage`
  ;[1 0.9205 0.3716] Add functionality for giving these effects to enemies within an array
)

(event `/Game/Classes/AI/BPI_ModifierBehaviour.Add Virus Damage`
  ;[1 0.9205 0.3716] Add functionality for giving these effects to enemies within an array
  (set `self.CanInflictVirusDamage` true)
  (`SceneComponent.SetVisibility` (`self.VirusDmg`) true true)
  (for _array_element (`self.EnemiesInRange`)
    (if (`self.CanInflictVirusDamage`)
      (`/Engine/EditorBlueprintResources/StandardMacros.IsValid` _array_element
        (:`Is Valid`
          (message `/Game/Classes/AI/BPI_AoeEffects.AI Virus Damage` _array_element (`self.VirusDamage`) (`self.VirusDamageRate`)))))))

(fn `UserConstructionScript`)