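; Gunner tower structure that automatically shoots enemies in range and supports damage upgrades.
; Once built it swaps the ghost mesh for the real one, scales its range trigger and tracks overlapping BPI_AISettings actors in an array.
; Each tick it checks the first enemy and, when the fire timer allows, spawns BP_Projectile carrying its damage stats.
; Blunt, pierce and virus upgrades reveal their meshes and deduct player resources; base damage upgrades only add damage.
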(event `/Game/Classes/Buildings/Interfaces/BPI_StructureStatus.StructureBuilt`
  (set `self.CanAttack` true)
  (`SceneComponent.SetVisibility` (`self.GhostStructure`) false true)
  (`SceneComponent.SetVisibility` (`self.MainStruct`) true false)
  (`self.ScaleTriggerToSize` (`self.TowerRangeTrigger`))
  (set `self.AmBuilt` true))

(event `self.ReceiveBeginPlay`
  (`parent.ReceiveBeginPlay`)
  (`SceneComponent.SetVisibility` (`self.VirusDmg`) false true)
  (`SceneComponent.SetVisibility` (`self.BluntDmg`) false true)
  (`SceneComponent.SetVisibility` (`self.PierceDmg`) false true)
  (`SceneComponent.SetVisibility` (`self.MainStruct`) false true))

(event `/Game/Classes/AI/BPI_ModifierBehaviour.Increase Blunt Damage`
  (set `self.BluntDamage` (+ (`self.BluntDamage`) 30.0))
  (`SceneComponent.SetVisibility` (`self.BluntDmg`) true true)
  (`/Game/Classes/Player/BP_PlayerPawn.ResourceDeduction` (`self.PlayerPawn`) (`/Game/Classes/GameFiles/BP_GameModeMain.BluntModCost` (`self.GameMode`))))

(event `self.ReceiveTick`
  (params (DeltaSeconds :type "Float (single-precision)"))
  (`parent.ReceiveTick` 0.0)
  (`self.CheckEnemies`))

(event `/Game/Classes/AI/BPI_ModifierBehaviour.Increase Pierce Damage`
  (set `self.PierceDamage` (+ (`self.PierceDamage`) 30.0))
  (`SceneComponent.SetVisibility` (`self.PierceDmg`) true true)
  (`/Game/Classes/Player/BP_PlayerPawn.ResourceDeduction` (`self.PlayerPawn`) (`/Game/Classes/GameFiles/BP_GameModeMain.PierceModCost` (`self.GameMode`))))

(event `/Game/Classes/AI/BPI_ModifierBehaviour.Increase Base Damage`
  (set `self.BaseDamage` (+ (`self.BaseDamage`) 10.0)))

(event `self.TowerRangeTrigger.OnComponentBeginOverlap`
  (params (OverlappedComponent :type "PrimitiveComponent Object Reference") (OtherActor :type "Actor Object Reference") (OtherComp :type "PrimitiveComponent Object Reference") (OtherBodyIndex :type Integer) (bFromSweep :type Boolean) (SweepResult :type "HitResult Structure (by ref)"))
  (`self.AddRemoveEnemy` true OtherActor))

(event `/Game/Classes/AI/BPI_ModifierBehaviour.Add Virus Damage`
  (if (not (`self.CanInflictVirusDamage`))
    (set `self.CanInflictVirusDamage` true)
    (`SceneComponent.SetVisibility` (`self.VirusDmg`) true true)
    (`/Game/Classes/Player/BP_PlayerPawn.ResourceDeduction` (`self.PlayerPawn`) (`/Game/Classes/GameFiles/BP_GameModeMain.VirusModCost` (`self.GameMode`)))))

(event `self.TowerRangeTrigger.OnComponentEndOverlap`
  (params (OverlappedComponent :type "PrimitiveComponent Object Reference") (OtherActor :type "Actor Object Reference") (OtherComp :type "PrimitiveComponent Object Reference") (OtherBodyIndex :type Integer))
  (`self.AddRemoveEnemy` false OtherActor))

(event `self.BuildingRange.OnComponentBeginOverlap`
  (params (OverlappedComponent :type "PrimitiveComponent Object Reference") (OtherActor :type "Actor Object Reference") (OtherComp :type "PrimitiveComponent Object Reference") (OtherBodyIndex :type Integer) (bFromSweep :type Boolean) (SweepResult :type "HitResult Structure (by ref)")))

(event `self.BuildingRange.OnComponentHit`
  (params (HitComponent :type "PrimitiveComponent Object Reference") (OtherActor :type "Actor Object Reference") (OtherComp :type "PrimitiveComponent Object Reference") (NormalImpulse :type "Vector Structure") (Hit :type "HitResult Structure (by ref)")))

(fn `AddRemoveEnemy`
  (params (InRange :type Boolean) (Actor :type "Actor Object Reference"))
  (`/Engine/EditorBlueprintResources/StandardMacros.IsValid` Actor
    (:`Is Valid`
      (if (`KismetSystemLibrary.DoesImplementInterface` Actor "/Game/Classes/Buildings/Interfaces/BPI_AISettings.BPI_AISettings_C")
        (if InRange
          (`KismetArrayLibrary.Array_Add` (`self.EnemyArray`) Actor)
          (else
            (`KismetArrayLibrary.Array_RemoveItem` (`self.EnemyArray`) Actor)))
        (else
          (`KismetSystemLibrary.PrintString` "No Interface Found"))))))

(fn `CheckEnemies`
  (bind _output (`|GetArrayItem` (`self.EnemyArray`)))
  (if (> (`KismetArrayLibrary.Array_Length` (`self.EnemyArray`)) 0)
    (if (>= (`KismetSystemLibrary.GetGameTimeInSeconds`) (`self.NewTime`))
      (`/Engine/EditorBlueprintResources/StandardMacros.IsValid` _output
        (:`Is Valid`
          (`self.Shoot Projectile` _output (`SceneComponent.K2_GetComponentLocation` (`self.GetComponentByClass` _output "/Game/Classes/Components/TargetComponentV2.TargetComponentV2_C")))
          (set `self.NewTime` (+ (`KismetSystemLibrary.GetGameTimeInSeconds`) (`self.FireRate`))))))))

(fn `Shoot Projectile`
  (params (ProjectileTarget :type "Actor Object Reference") (TargetLocation :type "Vector Structure"))
  (if (`self.CanAttack`)
    (`|SpawnActorFromClass` "/Game/Classes/Buildings/Attacks/BP_Projectile.BP_Projectile_C" (`KismetMathLibrary.MakeTransform` (`SceneComponent.K2_GetComponentLocation` (`self.ShotOrigin`))) "Undefined" "OverrideRootScale" null ProjectileTarget (`self.BaseDamage`) (`self.PierceDamage`) (`self.BluntDamage`) (`self.VirusDamage`) (`self.CanInflictVirusDamage`) (`self.VirusDamageRate`) TargetLocation self null)))

(fn `UserConstructionScript`)