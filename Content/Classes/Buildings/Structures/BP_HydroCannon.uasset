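; BP_HydroCannon is a buildable defensive tower that shoots mortar projectiles at enemies in range, spending stored energy per shot.
; On construction it swaps the ghost mesh for the real one, enables attacking and initiates linked energy plants.
; A trigger sphere tracks BPI_AISettings actors; Tick fires at the first one on a timed interval.
; Blunt, pierce and virus mods charge resources, grow indicator components and, like base damage, feed into each projectile.
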(event `/Game/Classes/Buildings/Interfaces/BPI_StructureStatus.StructureBuilt`
  (set `self.CanAttack` true)
  (`SceneComponent.SetVisibility` (`self.GhostStructure`) false false)
  (`SceneComponent.SetVisibility` (`self.MainStructure`) true false)
  (`self.ScaleTriggerToSize` (`self.TowerRangeTrigger`))
  (set `self.AmBuilt` true)
  (for _array_element (`self.EnergyPlantRef`)
    (bind _asbp_energy_plant (cast `/Game/Classes/Buildings/Structures/BP_EnergyPlant` _array_element))
    (`self.StructureEnergyInitiate` _asbp_energy_plant)))

(event `self.ReceiveBeginPlay`
  (`parent.ReceiveBeginPlay`)
  (`SceneComponent.SetVisibility` (`self.BluntDmg`) false false)
  (`SceneComponent.SetVisibility` (`self.PierceDmg`) false false)
  (`SceneComponent.SetVisibility` (`self.VirusDmg`) false false)
  (`SceneComponent.SetVisibility` (`self.MainStructure`) false false))

(event `self.ReceiveTick`
  (params (DeltaSeconds :type "Float (single-precision)"))
  (`parent.ReceiveTick` 0.0)
  (`self.CheckEnemies`))

(event `/Game/Classes/AI/BPI_ModifierBehaviour.Increase Blunt Damage`
  (bind _bluntdmg (`self.BluntDmg`))
  (set `self.BluntDamage` (+ (`self.BluntDamage`) 30.0))
  (`SceneComponent.SetVisibility` _bluntdmg true true)
  (`SceneComponent.SetWorldScale3D` _bluntdmg (+ (`SceneComponent.K2_GetComponentScale` _bluntdmg) (0.15 0.15 0.15)))
  (`/Game/Classes/Player/BP_PlayerPawn.ResourceDeduction` (`self.PlayerPawn`) (`/Game/Classes/GameFiles/BP_GameModeMain.BluntModCost` (`self.GameMode`))))

(event `/Game/Classes/AI/BPI_ModifierBehaviour.Increase Pierce Damage`
  (bind _piercedmg (`self.PierceDmg`))
  (set `self.PierceDamage` (+ (`self.PierceDamage`) 30.0))
  (`SceneComponent.SetVisibility` _piercedmg true true)
  (`SceneComponent.SetWorldScale3D` _piercedmg (+ (`SceneComponent.K2_GetComponentScale` _piercedmg) (0.15 0.15 0.15)))
  (`/Game/Classes/Player/BP_PlayerPawn.ResourceDeduction` (`self.PlayerPawn`) (`/Game/Classes/GameFiles/BP_GameModeMain.PierceModCost` (`self.GameMode`))))

(event `/Game/Classes/AI/BPI_ModifierBehaviour.Increase Base Damage`
  (set `self.BaseDamage` (+ (`self.BaseDamage`) 10.0)))

(event `self.TowerRangeTrigger.OnComponentBeginOverlap`
  (params (OverlappedComponent :type "PrimitiveComponent Object Reference") (OtherActor :type "Actor Object Reference") (OtherComp :type "PrimitiveComponent Object Reference") (OtherBodyIndex :type Integer) (bFromSweep :type Boolean) (SweepResult :type "HitResult Structure (by ref)"))
  (`self.AddRemoveEnemy` true OtherActor))

(event `/Game/Classes/AI/BPI_ModifierBehaviour.Add Virus Damage`
  (bind _virusdmg (`self.VirusDmg`))
  (if (not (`self.CanInflictVirusDamage`))
    (set `self.CanInflictVirusDamage` true)
    (`SceneComponent.SetVisibility` _virusdmg true true)
    (`SceneComponent.SetWorldScale3D` _virusdmg (+ (`SceneComponent.K2_GetComponentScale` _virusdmg) (0.15 0.15 0.15)))
    (`/Game/Classes/Player/BP_PlayerPawn.ResourceDeduction` (`self.PlayerPawn`) (`/Game/Classes/GameFiles/BP_GameModeMain.VirusModCost` (`self.GameMode`)))))

(event `self.TowerRangeTrigger.OnComponentEndOverlap`
  (params (OverlappedComponent :type "PrimitiveComponent Object Reference") (OtherActor :type "Actor Object Reference") (OtherComp :type "PrimitiveComponent Object Reference") (OtherBodyIndex :type Integer))
  (`self.AddRemoveEnemy` false OtherActor))

(fn `AddRemoveEnemy`
  (params (InRange :type Boolean) (Actor :type "Actor Object Reference"))
  (`/Engine/EditorBlueprintResources/StandardMacros.IsValid` Actor
    (:`Is Valid`
      (if (`KismetSystemLibrary.DoesImplementInterface` Actor "/Game/Classes/Buildings/Interfaces/BPI_AISettings.BPI_AISettings_C")
        (if InRange
          (`KismetArrayLibrary.Array_Add` (`self.EnemyArray`) Actor)
          (else
            (`KismetArrayLibrary.Array_RemoveItem` (`self.EnemyArray`) Actor)))
        (else
          (`KismetSystemLibrary.PrintString` "No Interface Found"))))))

(fn `CheckEnemies`
  (bind _output (`|GetArrayItem` (`self.EnemyArray`)))
  (if (> (`KismetArrayLibrary.Array_Length` (`self.EnemyArray`)) 0)
    (if (>= (`KismetSystemLibrary.GetGameTimeInSeconds`) (`self.NewTime`))
      (`/Engine/EditorBlueprintResources/StandardMacros.IsValid` _output
        (:`Is Valid`
          (`self.Shoot Projectile` _output)
          (set `self.NewTime` (+ (`KismetSystemLibrary.GetGameTimeInSeconds`) (`self.FireRate`))))))))

(fn `Shoot Projectile`
  (params (`Projectile Target` :type "Actor Object Reference"))
  (if (>= (`/Game/Classes/Components/CBP_EnergyComponent.CurrentEnergy` (`self.CBP_EnergyComponent`)) (`self.EnergyDeduct`))
    (if (`self.CanAttack`)
      (`|SpawnActorFromClass` "/Game/Classes/Buildings/Attacks/BP_MortarProjectile.BP_MortarProjectile_C" (`KismetMathLibrary.MakeTransform` (`SceneComponent.K2_GetComponentLocation` (`self.ShotOrigin`))) "Undefined" "OverrideRootScale" null `Projectile Target` (`self.RangedTowerDamage`) (`self.BluntDamage`) (`self.PierceDamage`) (`self.BaseDamage`) (`self.VirusDamage`) (`self.VirusDamageRate`) (`self.CanInflictVirusDamage`) null)
      (`/Game/Classes/Components/CBP_EnergyComponent.Deduct` (`self.CBP_EnergyComponent`) (`self.EnergyDeduct`)))))

(fn `UserConstructionScript`)