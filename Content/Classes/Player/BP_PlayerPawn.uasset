(event `self.ReceiveBeginPlay`
  (bind _returnvalue (`GameplayStatics.GetPlayerController` 0))
  (`|ExecutionSequence`
    (:`then_0`
      (bind _returnvalue_2 (`|CreateWidget` "/Game/Classes/UI/WBP_Resources.WBP_Resources_C" _returnvalue))
      (bind _output_get (set `self.HUD_Resources` _returnvalue_2))
      (`/Engine/EditorBlueprintResources/StandardMacros.IsValid` _output_get
        (:`Is Valid`
          (`UserWidget.AddToViewport` _output_get 0))))
    (:`then_1`
      (bind _returnvalue_3 (`|CreateWidget` "/Game/Classes/UI/WBP_Lives.WBP_Lives_C" _returnvalue))
      (bind _output_get_2 (set `self.HUD_Lives` _returnvalue_3))
      (`/Engine/EditorBlueprintResources/StandardMacros.IsValid` _output_get_2
        (:`Is Valid`
          (`UserWidget.AddToViewport` _output_get_2 0))))
    (:`then_2`
      (bind _returnvalue_4 (`|CreateWidget` "/Game/Classes/UI/WBP_BuildTowerV2.WBP_BuildTowerV2_C"))
      (bind _output_get_3 (set `self.HUD_BuildTowers` _returnvalue_4))
      (`|ExecutionSequence`
        (:`then_0`
          (`UserWidget.AddToViewport` _output_get_3 0))
        (:`then_1`
          (`/Game/Classes/UI/WBP_BuildTowerV2.Construct Base` _output_get_3))))))

(event `self.ReceiveTick`
  (params (DeltaSeconds :type "Float (single-precision)"))
  (bind (_hitresult _returnvalue) (`PlayerController.GetHitResultUnderCursorByChannel` (`GameplayStatics.GetPlayerController` 0) "TraceTypeQuery1" true))
  (`|ExecutionSequence`
    (:`then_0`
      (if (`self.CanMoveCamera`)
        (bind _output_get (set `self.Direction` (`self.Get Direction`)))
        (`self.K2_AddActorWorldOffset` (`self.Apply Directional Movement`))))
    (:`then_1`
      ;[0.009803 0.2538 0.6927 1 35] Building Functionality
      ;;[0.8594 0.3613 0.1794] Set Building Location
      (if (`self.IsBuilding`)
        (if _returnvalue
          (`self.K2_SetActorLocation` (`self.ActorToBuild`) (`.Location` (`GameplayStatics.BreakHitResult` _hitresult)) false false))))))

(event `InputAction|CancelBuild`
  (params (Key :type "Key Structure"))
  ;[0.009803 0.2538 0.6927 1 35] Building Functionality
  ;;[0 0.8146 1] Build Inputs
  (:`Pressed`
    (if (`self.IsBuilding`)
      (set `self.CanBuild` false)
      (set `self.IsBuilding` false)
      ;;[0.2934 0.191 1] Remove actor for building
      (`self.K2_DestroyActor` (`self.ActorToBuild`) :!label _label))))

(event `InputAction|Build`
  (params (Key :type "Key Structure"))
  (bind _returnvalue (`GameplayStatics.GetObjectClass` (`self.ActorToBuild`)))
  ;[0.009803 0.2538 0.6927 1 35] Building Functionality
  ;;[0 0.8146 1] Build Inputs
  (:`Pressed`
    (if (`self.CanBuild`)
      (set `self.IsBuilding` false)
      (`|SpawnActorFromClass` _returnvalue (`KismetMathLibrary.MakeTransform` (`.Location` (`GameplayStatics.BreakHitResult` (`PlayerController.GetHitResultUnderCursorByChannel` (`GameplayStatics.GetPlayerController` 0) "TraceTypeQuery1" true)))) "Undefined" "OverrideRootScale" null null)
      (`|ExecutionSequence`
        (:`then_0`
          (set `self.CanBuild` false)
          (goto _label))
        (:`then_1`
          ;;[1 0.7138 0.3712] Resource Deduction
          (if (== _returnvalue "/Game/Classes/Buildings/Structures/BP_B_Gunner.BP_B_Gunner_C")
            (`self.ResourceDeduction` (`self.Gunner Cost`))
            (`/Game/Classes/UI/WBP_Resources.Update Resource` (`self.HUD_Resources`) :!label _label_2)))
        (:`then_2`
          (if (== _returnvalue "/Game/Classes/Buildings/Structures/BP_B_HydroCannon.BP_B_HydroCannon_C")
            (`self.ResourceDeduction` (`self.Hydro Cost`))
            (goto _label_2)))
        (:`then_3`
          (if (== _returnvalue "/Game/Classes/Buildings/Structures/BP_B_Rectifier.BP_B_Rectifier_C")
            (`self.ResourceDeduction` (`self.Rectifier Cost`))
            (goto _label_2)))))))

(event `Add Building To Mouse Position`
  (params (ActorToBuild :type "Actor Class Reference"))
  ;[0.009803 0.2538 0.6927 1 35] Building Functionality
  ;;[0.3501 0.9302 1] OnButtonAddBuilding
  (set `self.CanBuild` true)
  (set `self.IsBuilding` true)
  (bind _returnvalue (`|SpawnActorFromClass` ActorToBuild (`KismetMathLibrary.MakeTransform` (`.Location` (`GameplayStatics.BreakHitResult` (`PlayerController.GetHitResultUnderCursorByChannel` (`GameplayStatics.GetPlayerController` 0) "TraceTypeQuery1" true)))) "Undefined" "OverrideRootScale" null null))
  (set `self.ActorToBuild` _returnvalue))

(fn `Apply Directional Movement`
  (returns (DirectionalMovement :type "Vector Structure"))
  (bind _up (`self.Get Up Direction`))
  (bind _down (`self.Get Down Direction`))
  (bind _right (`self.Get Right Direction`))
  (bind _left (`self.Get Left Direction`))
  (return (select `/Game/Classes/Player/BP_E_PlayerDirection` (`self.Direction`) :`NewEnumerator1` (* (`self.Get Up Direction`) (`self.CameraSpeed_full`)) :`NewEnumerator2` (* (`self.Get Down Direction`) (`self.CameraSpeed_full`)) :`NewEnumerator3` (* (`self.Get Left Direction`) (`self.CameraSpeed_full`)) :`NewEnumerator4` (* (`self.Get Right Direction`) (`self.CameraSpeed_full`)) :`NewEnumerator5` (* (+ _up _left) (`self.CameraSpeed_Diagonal`)) :`NewEnumerator6` (* (+ _up _right) (`self.CameraSpeed_Diagonal`)) :`NewEnumerator7` (* (+ _down _left) (`self.CameraSpeed_Diagonal`)) :`NewEnumerator8` (* (+ _down _right) (`self.CameraSpeed_Diagonal`)))))

(fn `Get Direction`
  (returns (Direction :type "/Game/Classes/Player/BP_E_PlayerDirection Enum"))
  (bind _returnvalue (`GameplayStatics.GetPlayerController` 0))
  (bind _returnvalue_2 (`GameplayStatics.GetPlayerController` 0))
  (bind _returnvalue_3 (`GameplayStatics.GetPlayerController` 0))
  (bind _returnvalue_4 (`GameplayStatics.GetPlayerController` 0))
  (bind _locationx (`PlayerController.GetMousePosition` _returnvalue))
  (bind _locationx_2 (`PlayerController.GetMousePosition` (`GameplayStatics.GetPlayerController` 0)))
  (bind _locationx_3 (`PlayerController.GetMousePosition` (`GameplayStatics.GetPlayerController` 0)))
  (bind _locationx_4 (`PlayerController.GetMousePosition` (`GameplayStatics.GetPlayerController` 0)))
  (bind (_locationx_5 _locationy) (`PlayerController.GetMousePosition` (`GameplayStatics.GetPlayerController` 0)))
  (bind (_locationx_6 _locationy_2) (`PlayerController.GetMousePosition` _returnvalue_2))
  (bind _locationx_7 (`PlayerController.GetMousePosition` _returnvalue_3))
  (bind _locationx_8 (`PlayerController.GetMousePosition` _returnvalue_4))
  (bind _returnvalue_5 (`KismetMathLibrary.Conv_IntToDouble` (`PlayerController.GetViewportSize` _returnvalue)))
  (bind _returnvalue_6 (`KismetMathLibrary.Conv_IntToDouble` (`.SizeY` (`PlayerController.GetViewportSize` _returnvalue_2))))
  (bind _returnvalue_7 (`KismetMathLibrary.Conv_IntToDouble` (`PlayerController.GetViewportSize` _returnvalue_3)))
  (bind _returnvalue_8 (`KismetMathLibrary.Conv_IntToDouble` (`PlayerController.GetViewportSize` _returnvalue_4)))
  (if (and (>= _locationy 0.0) (<= _locationy (`self.ScreenBorderBuffer`)))
    (if (and (>= _locationx_4 0.0) (<= _locationx_4 (`self.ScreenBorderBuffer`)))
      (return "NewEnumerator5")
      (elif (and (<= _locationx_8 _returnvalue_8) (>= _locationx_8 (- _returnvalue_8 (`self.ScreenBorderBuffer`))))
        (return "NewEnumerator6")
        (else
          (return "NewEnumerator1"))))
    (elif (and (<= _locationy_2 _returnvalue_6) (>= _locationy_2 (- _returnvalue_6 (`self.ScreenBorderBuffer`))))
      (if (and (>= _locationx_2 0.0) (<= _locationx_2 (`self.ScreenBorderBuffer`)))
        (return "NewEnumerator7")
        (elif (and (<= _locationx _returnvalue_5) (>= _locationx (- _returnvalue_5 (`self.ScreenBorderBuffer`))))
          (return "NewEnumerator8")
          (else
            (return "NewEnumerator2"))))
      (elif (and (>= _locationx_3 0.0) (<= _locationx_3 (`self.ScreenBorderBuffer`)))
        (return "NewEnumerator3")
        (elif (and (<= _locationx_7 _returnvalue_7) (>= _locationx_7 (- _returnvalue_7 (`self.ScreenBorderBuffer`))))
          (return "NewEnumerator4")
          (else
            (return "NewEnumerator0")))))))

(fn `Lose Game`
  (`/Engine/EditorBlueprintResources/StandardMacros.DoOnce` false
    (:`Completed`
      (`KismetSystemLibrary.PrintString` "You Lose")
      (return))))

(fn `ResourceCheck`
  (params (ButtonClicked :type "Button Object Reference"))
  (returns (CanBuild :type Boolean))
  (if (== ButtonClicked (`/Game/Classes/UI/WBP_BuildTowerV2.Button_Gunner` (`self.HUD_BuildTowers`)))
    (return (>= (`self.Resources`) (`self.Gunner Cost`)))
    (elif (== ButtonClicked (`/Game/Classes/UI/WBP_BuildTowerV2.Button_HydroCannon` (`self.HUD_BuildTowers`)))
      (return (>= (`self.Resources`) (`self.Hydro Cost`)))
      (elif (== ButtonClicked (`/Game/Classes/UI/WBP_BuildTowerV2.Button_Rectifier` (`self.HUD_BuildTowers`)))
        (return (>= (`self.Resources`) (`self.Rectifier Cost`)))))))

(fn `ResourceDeduction`
  (params (Cost :type Integer))
  (set `self.Resources` (- (`self.Resources`) Cost)))

(fn `Update Resources`
  (set `/Game/Classes/UI/WBP_Resources.ResourceText` (`KismetTextLibrary.Conv_IntToText` (`self.Resources`)) (`self.HUD_Resources`))
  (return))

(fn `UserConstructionScript`)