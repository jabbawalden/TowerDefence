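; Enemy AI character that follows a spline and awards its held resources to the player on death.
; On BeginPlay it scales speed and resistances by the game mode's difficulty multiplier, copying resistances into CBP_Health.
; Events handle slows, resistance debuffs, an affliction counter and heal/virus visuals; virus damage repeats via a timeline resized to the attack rate.
; Resistance debuffs change only the AI's own variables, never re-copying them to the health component.
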(event `self.ReceiveBeginPlay`
  ;[0 1 0.5223] AI Setup
  (`self.IncreaseDifficulty`)
  (`self.InitiateStats`)
  (`KismetSystemLibrary.Delay` 0.1)
  (`self.Follow Spline`)
  (`SceneComponent.SetVisibility` (`self.VirusAffected`) false false)
  (`SceneComponent.SetVisibility` (`self.HealEmitterStatic`) false false))

(event `/Game/Classes/AI/BPI_AoeEffects.AI Slow Down`
  (params (`Slow down severity` :type "Float (single-precision)"))
  (bind _charactermovement (`self.CharacterMovement`))
  ;[1 0.7303 0.2197] Slow down behaviour AOE
  (set `CharacterMovementComponent.MaxWalkSpeed` (/ (`CharacterMovementComponent.MaxWalkSpeed` _charactermovement) `Slow down severity`) _charactermovement))

(event `/Game/Classes/AI/BPI_Emitters.HealEmitter`
  (`SceneComponent.SetVisibility` (`self.HealEmitterStatic`) true true)
  (`KismetSystemLibrary.Delay` 0.4)
  (`SceneComponent.SetVisibility` (`self.HealEmitterStatic`) false false))

(event `/Game/Classes/AI/BPI_AoeEffects.AI Resume Speed`
  ;[1 0.7303 0.2197] Slow down behaviour AOE
  (set `CharacterMovementComponent.MaxWalkSpeed` (`self.Default Walk Speed`) (`self.CharacterMovement`)))

(event `self.CBP_Health.CallDeath`
  (if (not (`/Game/Classes/Components/CBP_Health.Alive` (`self.CBP_Health`)))
    (`self.Death`)))

(event `/Game/Classes/AI/BPI_AoeEffects.AI Virus Damage`
  (params (VirusDamage :type "Float (single-precision)") (AttackRate :type "Float (single-precision)"))
  (bind _virusdamagerate (`self.VirusDamageRate`))
  ;[1 0.7303 0.2197] Virus damage behaviour
  (`SceneComponent.SetVisibility` (`self.VirusAffected`) true true)
  (set `self.CanVirusDamage` true)
  (`KismetSystemLibrary.PrintString` "Virus Damage Inflicted")
  (if (`self.CanVirusDamage`) :!label _label
    (`/Engine/EditorBlueprintResources/StandardMacros.IsValid` self
      (:`Is Valid`
        (`/Game/Classes/GameFiles/BP_FunctionLibrary.Deal Damage To Actor` self 0.0 0.0 0.0 VirusDamage)
        (`/Engine/EditorBlueprintResources/StandardMacros.IsValid` _virusdamagerate
          (:`Is Valid`
            (`TimelineComponent.SetTimelineLength` _virusdamagerate AttackRate)
            (`Timeline|VirusDamageRate` :!via `PlayFromStart`
              (:`Finished`
                (goto _label)))))))))

(event `/Game/Classes/AI/BPI_AoeEffects.AI Virus Damage Stop`
  ;[1 0.7303 0.2197] Virus damage behaviour
  (`SceneComponent.SetVisibility` (`self.VirusAffected`) false false)
  (set `self.CanVirusDamage` false)
  (goto _label))

(event `/Game/Classes/AI/BPI_AoeEffects.AI Reduce Blunt Resistance`
  (params (`Is True` :type Boolean) (ReductionAmount :type "Float (single-precision)"))
  (set `self.AI Reduced Blunt Resistance` (* ReductionAmount (`self.AI Blunt Resistance`)))
  (set `self.AI Default Blunt Resistance` (`self.AI Blunt Resistance`))
  (if `Is True`
    (set `self.AI Blunt Resistance` (`self.AI Reduced Blunt Resistance`))
    (else
      (set `self.AI Blunt Resistance` (`self.AI Default Blunt Resistance`)))))

(event `/Game/Classes/AI/BPI_AoeEffects.AI Reduce Pierce Resistance`
  (params (`Is True` :type Boolean) (ReductionAmount :type "Float (single-precision)"))
  (set `self.AI Reduced Pierce Resistance` (* ReductionAmount (`self.AI Pierce Resistance`)))
  (set `self.AI Default Pierce Resistance` (`self.AI Pierce Resistance`))
  (if `Is True`
    (set `self.AI Pierce Resistance` (`self.AI Reduced Pierce Resistance`))
    (else
      (set `self.AI Pierce Resistance` (`self.AI Default Pierce Resistance`)))))

(event `/Game/Classes/AI/BPI_AoeEffects.AI ADD Afflicted Counter`
  (`self.SetAfflictedCounter` true))

(event `/Game/Classes/AI/BPI_AoeEffects.AI SUB Afflicted Counter`
  (`self.SetAfflictedCounter` false))

(fn `Damage Recieved`
  (params (Damage :type "Float (double-precision)")))

(fn `Death`
  (bind _asbp_player_pawn (cast `/Game/Classes/Player/BP_PlayerPawn` (`GameplayStatics.GetPlayerPawn` 0)))
  (set `/Game/Classes/Player/BP_PlayerPawn.Resources` (+ (`/Game/Classes/Player/BP_PlayerPawn.Resources` _asbp_player_pawn) (`self.ResourcesHeld`)) _asbp_player_pawn)
  (`/Game/Classes/UI/WBP_Resources.Update Resource` (`/Game/Classes/Player/BP_PlayerPawn.HUD_Resources` _asbp_player_pawn))
  (`self.K2_DestroyActor`))

(fn `IncreaseDifficulty`
  (bind _asbp_game_mode_main (cast `/Game/Classes/GameFiles/BP_GameModeMain` (`GameplayStatics.GetGameMode`)))
  (`|ExecutionSequence`
    (:`then_0`
      (bind _difficultymultiplier (`/Game/Classes/GameFiles/BP_GameModeMain.DifficultyMultiplier` _asbp_game_mode_main))
      (bind _output_get (set `self.Default Walk Speed` (* (`self.Default Walk Speed`) _difficultymultiplier))))
    (:`then_1`
      (set `self.AI Pierce Resistance` (* (`self.AI Pierce Resistance`) _difficultymultiplier)))
    (:`then_2`
      (set `self.AI Blunt Resistance` (* (`self.AI Blunt Resistance`) _difficultymultiplier)))))

(fn `InitiateStats`
  (bind _cbp_health (`self.CBP_Health`))
  (set `/Game/Classes/Components/CBP_Health.Pierce Resistance` (`self.AI Pierce Resistance`) _cbp_health)
  (set `/Game/Classes/Components/CBP_Health.Blunt Resistance` (`self.AI Blunt Resistance`) _cbp_health)
  (set `CharacterMovementComponent.MaxWalkSpeed` (`self.Default Walk Speed`) (`self.CharacterMovement`)))

(fn `SetAfflictedCounter`
  (params (IsAdding :type Boolean))
  (if IsAdding
    (set `self.AfflictedCounter` (+ (`self.AfflictedCounter`) 1))
    (else
      (set `self.AfflictedCounter` (- (`self.AfflictedCounter`) 1)))))

(fn `UserConstructionScript`)