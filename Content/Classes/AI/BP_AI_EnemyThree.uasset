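; Healer enemy AI that follows a spline, supports nearby enemies and awards its held resources to the player on death.
; Tick periodically finds the lowest-health enemy inside HealRange, calls Heal on it (currently passing zero) and triggers its heal emitter through BPI_Emitters.
; Interface events handle slowdowns, an affliction counter and virus damage, which repeats via a timeline resized to the attack rate.
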(event `self.ReceiveBeginPlay`
  (`SceneComponent.SetVisibility` (`self.VirusAffected`) false false)
  (`SceneComponent.SetVisibility` (`self.HealEmitterStatic`) false false)
  (`self.InitiateStats`)
  (`KismetSystemLibrary.Delay` 0.1)
  (`self.Follow Spline`))

(event `self.CBP_Health.CallDeath`
  (if (not (`/Game/Classes/Components/CBP_HealthComponent.Alive` (`self.CBP_Health`)))
    (`self.Death`)))

(event `/Game/Classes/AI/BPI_AoeEffects.AI Slow Down`
  (params (`Slow down severity` :type "Float (single-precision)"))
  (bind _charactermovement (`self.CharacterMovement`))
  ;[1 0.9895 0.3272] Speed Changes Interface
  (set `CharacterMovementComponent.MaxWalkSpeed` (/ (`CharacterMovementComponent.MaxWalkSpeed` _charactermovement) `Slow down severity`) _charactermovement))

(event `/Game/Classes/AI/BPI_Emitters.HealEmitter`
  (`SceneComponent.SetVisibility` (`self.HealEmitterStatic`) true true)
  (`KismetSystemLibrary.Delay` 0.4)
  (`SceneComponent.SetVisibility` (`self.HealEmitterStatic`) false false))

(event `self.ReceiveTick`
  (params (DeltaSeconds :type "Float (single-precision)"))
  (bind _returnvalue (`KismetSystemLibrary.GetGameTimeInSeconds`))
  (if (<= (`self.NewTime`) _returnvalue)
    (set `self.NewTime` (+ _returnvalue (`self.TimeRate`)))
    (`self.Heal`)))

(event `/Game/Classes/AI/BPI_AoeEffects.AI Resume Speed`
  ;[1 0.9895 0.3272] Speed Changes Interface
  (set `CharacterMovementComponent.MaxWalkSpeed` (`self.Default Walk Speed`) (`self.CharacterMovement`)))

(event `/Game/Classes/AI/BPI_AoeEffects.AI Virus Damage`
  (params (VirusDamage :type "Float (single-precision)") (AttackRate :type "Float (single-precision)"))
  (bind _virusdamagerate (`self.VirusDamageRate`))
  ;[1 0.7303 0.2197] Virus damage behaviour
  (`SceneComponent.SetVisibility` (`self.VirusAffected`) true true)
  (set `self.Can Virus Damage` true)
  (if (`self.Can Virus Damage`) :!label _label
    (`/Engine/EditorBlueprintResources/StandardMacros.IsValid` self
      (:`Is Valid`
        (`/Game/Classes/GameFiles/BP_FunctionLibrary.Deal Damage To Actor` self 0.0 0.0 0.0 (* VirusDamage 2.0))
        (`/Engine/EditorBlueprintResources/StandardMacros.IsValid` _virusdamagerate
          (:`Is Valid`
            (`TimelineComponent.SetTimelineLength` _virusdamagerate AttackRate)
            (`Timeline|VirusDamageRate` :!via `PlayFromStart`
              (:`Finished`
                (goto _label)))))))))

(event `self.HealRange.OnComponentBeginOverlap`
  (params (OverlappedComponent :type "PrimitiveComponent Object Reference") (OtherActor :type "Actor Object Reference") (OtherComp :type "PrimitiveComponent Object Reference") (OtherBodyIndex :type Integer) (bFromSweep :type Boolean) (SweepResult :type "HitResult Structure (by ref)"))
  (`/Engine/EditorBlueprintResources/StandardMacros.IsValid` OtherActor
    (:`Is Valid`
      (if (`self.ActorHasTag` OtherActor "Enemy")
        (`KismetArrayLibrary.Array_Add` (`self.EnemyArray`) OtherActor)))))

(event `/Game/Classes/AI/BPI_AoeEffects.AI Virus Damage Stop`
  ;[1 0.7303 0.2197] Virus damage behaviour
  (`KismetSystemLibrary.PrintString` "Stop Virus")
  (`SceneComponent.SetVisibility` (`self.VirusAffected`) false false)
  (set `self.Can Virus Damage` false)
  (goto _label))

(event `self.HealRange.OnComponentEndOverlap`
  (params (OverlappedComponent :type "PrimitiveComponent Object Reference") (OtherActor :type "Actor Object Reference") (OtherComp :type "PrimitiveComponent Object Reference") (OtherBodyIndex :type Integer))
  (`/Engine/EditorBlueprintResources/StandardMacros.IsValid` OtherActor
    (:`Is Valid`
      (if (`self.ActorHasTag` OtherActor "Enemy")
        (`KismetArrayLibrary.Array_RemoveItem` (`self.EnemyArray`) OtherActor)))))

(event `/Game/Classes/AI/BPI_AoeEffects.AI ADD Afflicted Counter`
  (`self.SetAfflictedCounter` true))

(event `/Game/Classes/AI/BPI_AoeEffects.AI SUB Afflicted Counter`
  (`self.SetAfflictedCounter` false))

(fn `Damage Recieved`
  (params (Damage :type "Float (double-precision)")))

(fn `Death`
  (bind _asbp_player_pawn (cast `/Game/Classes/Player/BP_PlayerPawn` (`GameplayStatics.GetPlayerPawn` 0)))
  (set `/Game/Classes/Player/BP_PlayerPawn.Resources` (+ (`/Game/Classes/Player/BP_PlayerPawn.Resources` _asbp_player_pawn) (`self.ResourcesHeld`)) _asbp_player_pawn)
  (`/Game/Classes/UI/WBP_Resources.Update Resource` (`/Game/Classes/Player/BP_PlayerPawn.HUD_Resources` _asbp_player_pawn))
  (`self.K2_DestroyActor`))

(fn `Heal`
  (bind _actorinneedofheal (`self.ActorInNeedOfHeal`))
  (set `self.LowestHealth` 1.0)
  (for _array_element (`self.EnemyArray`)
    (`/Engine/EditorBlueprintResources/StandardMacros.IsValid` _array_element
      (:`Is Valid`
        (bind _healthpercent (`/Game/Classes/Components/CBP_HealthComponent.GetPercent` (`self.GetComponentByClass` _array_element "/Game/Classes/Components/CBP_HealthComponent.CBP_HealthComponent_C")))
        (if (< _healthpercent (`self.LowestHealth`))
          (set `self.LowestHealth` _healthpercent)
          (set `self.ActorInNeedOfHeal` _array_element)))))
  ;[1 1 1] If damage detected
  (if (< (`self.LowestHealth`) 1.0)
    (`/Game/Classes/Components/CBP_HealthComponent.Heal` (`self.GetComponentByClass` _actorinneedofheal "/Game/Classes/Components/CBP_HealthComponent.CBP_HealthComponent_C") 0.0)
    (if (`KismetSystemLibrary.DoesImplementInterface` _actorinneedofheal "/Game/Classes/AI/BPI_Emitters.BPI_Emitters_C")
      (message `/Game/Classes/AI/BPI_Emitters.HealEmitter` _actorinneedofheal))))

(fn `IncreaseDifficulty`
  (bind _asbp_game_mode_main (cast `/Game/Classes/GameFiles/BP_GameModeMain` (`GameplayStatics.GetGameMode`)))
  (`|ExecutionSequence`
    (:`then_0`
      (set `self.Default Walk Speed` (* (`self.Default Walk Speed`) (`/Game/Classes/GameFiles/BP_GameModeMain.DifficultyMultiplier` _asbp_game_mode_main))))))

(fn `InitiateStats`
  (set `CharacterMovementComponent.MaxWalkSpeed` (`self.Default Walk Speed`) (`self.CharacterMovement`)))

(fn `SetAfflictedCounter`
  (params (IsAdding :type Boolean))
  (if IsAdding
    (set `self.AfflictedCounter` (+ (`self.AfflictedCounter`) 1))
    (else
      (set `self.AfflictedCounter` (- (`self.AfflictedCounter`) 1)))))

(fn `UserConstructionScript`)