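; Base AI enemy that walks a spline path owned by its enemy system and can cost the player a life.
; FollowSpline moves to the current spline point with random XY jitter, while NextLocationIndex advances the index and continues until the last point.
; DeductLife decrements pawn lives, updates the lives widget, destroys the enemy and triggers GameLost on the last life.
; The older destination-actor movement chain is disconnected.
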(event `Follow Spline`
  ;[0.2817 0.6802 1] Move Functionality V2
  (bind _destination (`self.GetNextDestination`))
  (`|AIMoveTo` self _destination null))

(event `/Game/Classes/Buildings/Interfaces/BPI_AISettings.Next Location Index`
  ;[0.2817 0.6802 1] Move Functionality V2
  (bind _output_get (set `self.SPointDestination` (+ (`self.SPointDestination`) 1)))
  (if (not (== (`SplineComponent.GetNumberOfSplinePoints` (`/Game/Classes/WorldFiles/BP_EnemySystem.Spline` (`self.BP Enemy System`))) _output_get))
    (`self.Follow Spline`)))

(event `/Game/Classes/Buildings/Interfaces/BPI_AISettings.Set Enemy System Ref`
  (params (`BP Enemy System` :type "/Game/Classes/WorldFiles/BP_EnemySystem Object Reference"))
  ;[0.2817 0.6802 1] Move Functionality V2
  (set `self.BP Enemy System` `BP Enemy System`))

(event `AIMoveToNewLoc`
  (params (Class :type "Actor Class Reference"))
  ;[0 0 0] Move Functionality OLD
)

(fn `DeductLife`
  (bind _asbp_game_mode_main (cast `/Game/Classes/GameFiles/BP_GameModeMain` (`GameplayStatics.GetGameMode`)))
  (if (not (`/Game/Classes/GameFiles/BP_GameModeMain.Game Lost` _asbp_game_mode_main))
    (bind _asbp_player_pawn (cast `/Game/Classes/Player/BP_PlayerPawn` (`GameplayStatics.GetPlayerPawn` 0)))
    (bind _lives (`/Game/Classes/Player/BP_PlayerPawn.Lives` _asbp_player_pawn))
    (if (> _lives 1)
      (bind _returnvalue (- _lives 1))
      (set `/Game/Classes/Player/BP_PlayerPawn.Lives` _returnvalue _asbp_player_pawn)
      (else
        (set `/Game/Classes/Player/BP_PlayerPawn.Lives` _returnvalue _asbp_player_pawn)
        (bind _asbp_game_mode_main_2 (cast `/Game/Classes/GameFiles/BP_GameModeMain` (`GameplayStatics.GetGameMode`)))
        (`/Game/Classes/GameFiles/BP_GameModeMain.GameLost` _asbp_game_mode_main_2)))
    (bind _returnvalue_2 (`|CreateWidget` "/Game/Classes/UI/WBP_Lives.WBP_Lives_C" (`GameplayStatics.GetPlayerController` 0)))
    (`/Game/Classes/UI/WBP_Lives.Update Lives` _returnvalue_2)
    (`self.K2_DestroyActor`)))

(fn `GetNextDestination`
  (returns (Destination :type "Vector Structure"))
  (bind _returnvalue (`KismetMathLibrary.RandomFloatInRange` -70.0 70.0))
  (bind _spointdestination (`self.SPointDestination`))
  (bind _spline (`/Game/Classes/WorldFiles/BP_EnemySystem.Spline` (`self.BP Enemy System`)))
  (if (>= _spointdestination (`SplineComponent.GetNumberOfSplinePoints` _spline))
    (`self.DeductLife`)
    (`KismetSystemLibrary.PrintString` "Life Deducted")
    (else
      (`/Engine/EditorBlueprintResources/StandardMacros.IsValid` _spline
        (:`Is Valid`
          (return (+ (`SplineComponent.GetLocationAtDistanceAlongSpline` _spline (`SplineComponent.GetDistanceAlongSplineAtSplinePoint` _spline _spointdestination) "World") (`KismetMathLibrary.MakeVector` _returnvalue _returnvalue))))))))

(fn `UserConstructionScript`)