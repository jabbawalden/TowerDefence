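; BP_Ark is the Ark class, which tracks module upgrade progress toward enabling a launch.
; Filler upgrades add to the total point count, while necessity upgrades add to both the necessity and total counts.
; Each upgrade runs a check that only prints "Launch Enabled" when both counts exactly equal their maximums, with no further launch logic.
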(fn `CheckUpgradePoints`
  (if (== (`self.Current Necessity Points`) (`self.Max Necessity Points`))
    (if (== (`self.Current Total Upgrade Points`) (`self.Max Total Upgrade Points`))
      (`KismetSystemLibrary.PrintString` "Launch Enabled"))))

(fn `UpgradeFillerModule`
  (set `self.Current Total Upgrade Points` (+ (`self.Current Total Upgrade Points`) 1))
  (`self.CheckUpgradePoints`))

(fn `UpgradeNecessityModule`
  (set `self.Current Necessity Points` (+ (`self.Current Necessity Points`) 1))
  (set `self.Current Total Upgrade Points` (+ (`self.Current Total Upgrade Points`) 1))
  (`self.CheckUpgradePoints`))

(fn `UserConstructionScript`)